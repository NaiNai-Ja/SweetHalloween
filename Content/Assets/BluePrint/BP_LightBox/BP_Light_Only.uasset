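; BP_Light_Only is a light Blueprint that flickers continuously from BeginPlay.
; FlickeringLight waits a random time between MinTime and MaxTime, flip-flops Light between fixed dim and bright intensities, then calls itself again.
; The construction script applies the Intensity variable, which the flicker loop later overrides.
; An IsFlickering rep-notify sets LightStatus and restarts the loop, but its branch condition is hard-coded true.
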(event Custom|FlickeringLight
  (bind _light (Variables|Default|GetLight))
  (Utilities|FlowControl|RetriggerableDelay (Math|Random|RandomFloatinRange (Variables|Default|GetMinTime) (Variables|Default|GetMaxTime)))
  (Utilities|FlowControl|FlipFlop
    (:A
      (Rendering|Components|Light|SetIntensity _light 1.0)
      (CallFunction|FlickeringLight))
    (:B
      (Rendering|Components|Light|SetIntensity _light 1e+01)
      (CallFunction|FlickeringLight))))

(event EventBeginPlay
  (CallFunction|FlickeringLight))

(fn ConstructionScript
  (Rendering|Components|Light|SetIntensity (Variables|Default|GetLight) (Variables|Default|GetIntensity)))

(fn OnRepIsFlickering
  (if true
    (Variables|Default|SetLightStatus "NewEnumerator1")
    (CallFunction|FlickeringLight)
    (else
      (Variables|Default|SetLightStatus "NewEnumerator0")
      (CallFunction|FlickeringLight))))