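; Light box actor that updates the player's in-dark status through an overlap volume and can flicker its light.
; Entering clears the player's Indark flag only while IsFlickering is true; leaving sets it and calls LowerMind on the status component.
; BeginPlay reassigns IsFlickering to itself, and its RepNotify sets LightStatus and calls FlickeringLight.
; That event loops through a random retriggerable delay and FlipFlop, alternating dim and brighter intensities.
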(event OnComponentBeginOverlap(Box)
  (params (OverlappedComponent :type Primitive%20Component%20Object%20Reference) (OtherActor :type Actor%20Object%20Reference) (OtherComp :type Primitive%20Component%20Object%20Reference) (OtherBodyIndex :type Integer) (bFromSweep :type Boolean) (SweepResult :type Hit%20Result%20Structure%20%28by%20ref%29))
  (bind _asbp_third_person_character (Utilities|Casting|CastToBP_ThirdPersonCharacter OtherActor))
  (if (Variables|Default|GetIsFlickering)
    (Variables|/Game/ThirdPerson/Blueprints/BPC_PlayerStatus.BPC_PlayerStatus_C|SetIndark (Variables|/Game/ThirdPerson/Blueprints/BP_ThirdPersonCharacter.BP_ThirdPersonCharacter_C|GetBPC_PlayerStatus _asbp_third_person_character) false)
    (else
      (Variables|/Game/ThirdPerson/Blueprints/BPC_PlayerStatus.BPC_PlayerStatus_C|SetIndark (Variables|/Game/ThirdPerson/Blueprints/BP_ThirdPersonCharacter.BP_ThirdPersonCharacter_C|GetBPC_PlayerStatus _asbp_third_person_character) true))))

(event OnComponentEndOverlap(Box)
  (params (OverlappedComponent :type Primitive%20Component%20Object%20Reference) (OtherActor :type Actor%20Object%20Reference) (OtherComp :type Primitive%20Component%20Object%20Reference) (OtherBodyIndex :type Integer))
  (bind _asbp_third_person_character (Utilities|Casting|CastToBP_ThirdPersonCharacter OtherActor))
  (Variables|/Game/ThirdPerson/Blueprints/BPC_PlayerStatus.BPC_PlayerStatus_C|SetIndark (Variables|/Game/ThirdPerson/Blueprints/BP_ThirdPersonCharacter.BP_ThirdPersonCharacter_C|GetBPC_PlayerStatus _asbp_third_person_character) true)
  (Default|LowerMind (Variables|/Game/ThirdPerson/Blueprints/BP_ThirdPersonCharacter.BP_ThirdPersonCharacter_C|GetBPC_PlayerStatus _asbp_third_person_character)))

(event Custom|FlickeringLight
  (bind _light (Variables|Default|GetLight))
  (if (Variables|Default|GetIsFlickering)
    (Utilities|FlowControl|RetriggerableDelay (Math|Random|RandomFloatinRange (Variables|Default|GetMinTime) (Variables|Default|GetMaxTime)))
    (Utilities|FlowControl|FlipFlop
      (:A
        (Rendering|Components|Light|SetIntensity _light 1.0)
        (CallFunction|FlickeringLight))
      (:B
        (Rendering|Components|Light|SetIntensity _light 1e+01)
        (CallFunction|FlickeringLight)))))

(event Custom|CheckStateLights
  (switch Utilities|FlowControl|Switch|SwitchonEN_LightBoxStatus (Variables|Default|GetLightStatus)
    (:NewEnumerator0
      (Rendering|Components|Light|SetIntensity (Variables|Default|GetLight) 5e+01))
    (:NewEnumerator1
      (CallFunction|FlickeringLight))))

(event EventBeginPlay
  (Variables|Default|SetIsFlickering (Variables|Default|GetIsFlickering)))

(fn ConstructionScript
  (Rendering|Components|Light|SetIntensity (Variables|Default|GetLight) (Variables|Default|GetIntensity)))

(fn OnRepIsFlickering
  (if (Variables|Default|GetIsFlickering)
    (Variables|Default|SetLightStatus "NewEnumerator1")
    (CallFunction|FlickeringLight)
    (else
      (Variables|Default|SetLightStatus "NewEnumerator0")
      (CallFunction|FlickeringLight))))