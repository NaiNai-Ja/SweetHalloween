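; BP_Candy_2 is a floating candy pickup shown as a paper sprite that the player collects by interacting.
; Timeline playback alternates forward and reverse to bob the sprite, while sphere overlap with the player toggles custom depth stencil and an inner interact icon.
; CanInteract reports a completed objective to BP_GameManager, increments the inventory's candy count, plays a sound, calls SetKeyopacity on BP_MusicBoxKey, then destroys the actor.
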(event OnComponentBeginOverlap(Sphere)
  (params (OverlappedComponent :type Primitive%20Component%20Object%20Reference) (OtherActor :type Actor%20Object%20Reference) (OtherComp :type Primitive%20Component%20Object%20Reference) (OtherBodyIndex :type Integer) (bFromSweep :type Boolean) (SweepResult :type Hit%20Result%20Structure%20%28by%20ref%29))
  ;[1 1 1] Comment
  (if (== OtherActor (Game|GetPlayerCharacter 0))
    (Rendering|SetCustomDepthStencilValue (Variables|Default|GetPaperSprite) 1)
    (CallFunction|IconInneron)))

(event OnComponentEndOverlap(Sphere)
  (params (OverlappedComponent :type Primitive%20Component%20Object%20Reference) (OtherActor :type Actor%20Object%20Reference) (OtherComp :type Primitive%20Component%20Object%20Reference) (OtherBodyIndex :type Integer))
  ;[1 1 1] Comment
  (if (== OtherActor (Game|GetPlayerCharacter 0))
    (Rendering|SetCustomDepthStencilValue (Variables|Default|GetPaperSprite) 0)
    (CallFunction|IconInnerOff)))

(event Custom|PlayAni
  ;[1 1 1] Floating
  (bind _z_movemant (Timeline|Timeline PlayFromStart)
    (:Update
      (Transformation|SetRelativeLocation (Variables|Default|GetPaperSprite) _z_movemant false false))
    (:Finished
      (CallFunction|PlayReverse))))

(event Custom|Icon%20innerOn
  ;[1 1 1] Comment
  (Rendering|SetVisibility (Variables|Default|GetinnerInteractIcon) true false))

(event Custom|Icon%20innerOff
  ;[1 1 1] Comment
  (Rendering|SetVisibility (Variables|Default|GetinnerInteractIcon) false false))

(event Custom|PlayReverse
  ;[1 1 1] Floating
  (bind _z_movemant (Timeline|Timeline_0 ReverseFromEnd)
    (:Update
      (Transformation|SetRelativeLocation (Variables|Default|GetPaperSprite) _z_movemant false false))
    (:Finished
      (CallFunction|PlayAni))))

(event EventCanInteract
  (bind _as_player (Variables|Default|GetAs%20Player))
  (bind _bpc_inventory (Variables|/Game/ThirdPerson/Blueprints/BP_ThirdPersonCharacter.BP_ThirdPersonCharacter_C|GetBPC_Inventory _as_player))
  ;[1 1 1] Comment
  (Class|IObjective|CompletedObjective(Message) (Variables|Default|GetAs%20Game%20Manager) 9)
  (Variables|/Game/ThirdPerson/Blueprints/BPC_Inventory.BPC_Inventory_C|SetCandy _bpc_inventory (+ (Variables|/Game/ThirdPerson/Blueprints/BPC_Inventory.BPC_Inventory_C|GetCandy _bpc_inventory) 1))
  (Utilities|FlowControl|Delay 0.2)
  (Audio|PlaySound2D "/Game/Sounds/Forlay/SFX_PickupGhostPaper.SFX_PickupGhostPaper" 1.0 1.0 0.0 0 0)
  (bind _returnvalue (Actor|GetActorOfClass "/Game/Assets/BluePrint/BP_InteractObject/BP_InteractAll/BP_MusicBoxKey.BP_MusicBoxKey_C"))
  (Default|SetKeyopacity _returnvalue)
  (Actor|DestroyActor))

(event EventBeginPlay
  ;[1 1 1] Get player BP
  (CallFunction|PlayAni)
  (bind _asbp_third_person_character (Utilities|Casting|CastToBP_ThirdPersonCharacter (Game|GetPlayerCharacter 0)))
  (Variables|Default|SetAs%20Player _asbp_third_person_character)
  (bind _returnvalue (Actor|GetActorOfClass "/Game/ThirdPerson/Blueprints/BP_Objective/BP_GameManager.BP_GameManager_C"))
  (Variables|Default|SetAs%20Game%20Manager _returnvalue))

(fn ConstructionScript)