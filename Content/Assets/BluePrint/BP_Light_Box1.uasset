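; BP_Light_Box1 is a flickering light with a box volume that marks whether the player character is in darkness.
; Overlapping the box clears Indark on the character's BPCPlayerStatus whatever IsFine is, while leaving sets it and calls LowerMind.
; From BeginPlay, a looping random delay between MinTime and MaxTime drives a FlipFlop that alternates the light between dim and bright.
; The construction script applies the Intensity variable, and the FlickeringLights event is empty.
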(event OnComponentBeginOverlap(Box)
  (params (OverlappedComponent :type Primitive%20Component%20Object%20Reference) (OtherActor :type Actor%20Object%20Reference) (OtherComp :type Primitive%20Component%20Object%20Reference) (OtherBodyIndex :type Integer) (bFromSweep :type Boolean) (SweepResult :type Hit%20Result%20Structure%20%28by%20ref%29))
  (bind _asbp_third_person_character (Utilities|Casting|CastToBP_ThirdPersonCharacter OtherActor))
  (if (Variables|Default|GetIsFine)
    (Variables|/Game/ThirdPerson/Blueprints/BPC_PlayerStatus.BPC_PlayerStatus_C|SetIndark (Variables|/Game/ThirdPerson/Blueprints/BP_ThirdPersonCharacter.BP_ThirdPersonCharacter_C|GetBPC_PlayerStatus _asbp_third_person_character) false)
    (else
      (Variables|/Game/ThirdPerson/Blueprints/BPC_PlayerStatus.BPC_PlayerStatus_C|SetIndark (Variables|/Game/ThirdPerson/Blueprints/BP_ThirdPersonCharacter.BP_ThirdPersonCharacter_C|GetBPC_PlayerStatus _asbp_third_person_character) false))))

(event OnComponentEndOverlap(Box)
  (params (OverlappedComponent :type Primitive%20Component%20Object%20Reference) (OtherActor :type Actor%20Object%20Reference) (OtherComp :type Primitive%20Component%20Object%20Reference) (OtherBodyIndex :type Integer))
  (bind _asbp_third_person_character (Utilities|Casting|CastToBP_ThirdPersonCharacter OtherActor))
  (Variables|/Game/ThirdPerson/Blueprints/BPC_PlayerStatus.BPC_PlayerStatus_C|SetIndark (Variables|/Game/ThirdPerson/Blueprints/BP_ThirdPersonCharacter.BP_ThirdPersonCharacter_C|GetBPC_PlayerStatus _asbp_third_person_character) true)
  (Default|LowerMind (Variables|/Game/ThirdPerson/Blueprints/BP_ThirdPersonCharacter.BP_ThirdPersonCharacter_C|GetBPC_PlayerStatus _asbp_third_person_character)))

(event Custom|FlickeringLights)

(event EventBeginPlay
  (bind _light (Variables|Default|GetLight))
  (Utilities|FlowControl|RetriggerableDelay (Math|Random|RandomFloatinRange (Variables|Default|GetMinTime) (Variables|Default|GetMaxTime)) :!label _label)
  (Utilities|FlowControl|FlipFlop
    (:A
      (Rendering|Components|Light|SetIntensity _light 5.0)
      (goto _label))
    (:B
      (Rendering|Components|Light|SetIntensity _light 5e+01)
      (goto _label))))

(fn ConstructionScript
  (Rendering|Components|Light|SetIntensity (Variables|Default|GetLight) (Variables|Default|GetIntensity)))