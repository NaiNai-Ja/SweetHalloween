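; BP_keyTable is an interactable key pickup that adds its item to the player's inventory.
; A sphere overlap with the player shows the inner interact icon and changes the sprite's custom depth stencil value, reverting both on exit.
; CanInteract completes an objective message through BP_GameManager, plays the key sound, adds the item through BPCInventory, then destroys the actor after a short delay.
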(event OnComponentBeginOverlap(Sphere)
  (params (OverlappedComponent :type Primitive%20Component%20Object%20Reference) (OtherActor :type Actor%20Object%20Reference) (OtherComp :type Primitive%20Component%20Object%20Reference) (OtherBodyIndex :type Integer) (bFromSweep :type Boolean) (SweepResult :type Hit%20Result%20Structure%20%28by%20ref%29))
  ;[1 1 1] Comment
  (if (== OtherActor (Game|GetPlayerCharacter 0))
    (CallFunction|IconInneron)
    (Rendering|SetCustomDepthStencilValue (Variables|Default|GetPaperSprite) 1)))

(event OnComponentEndOverlap(Sphere)
  (params (OverlappedComponent :type Primitive%20Component%20Object%20Reference) (OtherActor :type Actor%20Object%20Reference) (OtherComp :type Primitive%20Component%20Object%20Reference) (OtherBodyIndex :type Integer))
  ;[1 1 1] Comment
  (if (== OtherActor (Game|GetPlayerCharacter 0))
    (CallFunction|IconInnerOff)
    (Rendering|SetCustomDepthStencilValue (Variables|Default|GetPaperSprite) 0)))

(event Custom|Icon%20innerOn
  ;[1 1 1] Comment
  (Rendering|SetVisibility (Variables|Default|GetinnerInteractIcon) true false))

(event Custom|Icon%20innerOff
  ;[1 1 1] Comment
  (Rendering|SetVisibility (Variables|Default|GetinnerInteractIcon) false false))

(event EventCanInteract
  ;[1 1 1] Comment
  (Class|IObjective|CompletedObjective(Message) (Variables|Default|GetAs%20Game%20Manager) 7)
  (Audio|PlaySound2D "/Game/Sounds/Forlay/SFX_GetKey.SFX_GetKey" 1.0 1.0 0.0 0 0)
  (Default|AddItemtoInventory (Variables|/Game/ThirdPerson/Blueprints/BP_ThirdPersonCharacter.BP_ThirdPersonCharacter_C|GetBPC_Inventory (Variables|Default|GetAs%20Player)) (Variables|Default|GetItem))
  (Utilities|FlowControl|Delay 0.2)
  (Actor|DestroyActor))

(event EventBeginPlay
  ;[1 1 1] Get player BP
  (bind _asbp_third_person_character (Utilities|Casting|CastToBP_ThirdPersonCharacter (Game|GetPlayerCharacter 0)))
  (Variables|Default|SetAs%20Player _asbp_third_person_character)
  (bind _returnvalue (Actor|GetActorOfClass "/Game/ThirdPerson/Blueprints/BP_Objective/BP_GameManager.BP_GameManager_C"))
  (Variables|Default|SetAs%20Game%20Manager _returnvalue))

(fn ConstructionScript)