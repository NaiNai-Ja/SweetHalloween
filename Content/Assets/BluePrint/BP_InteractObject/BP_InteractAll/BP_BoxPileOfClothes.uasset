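; BP_BoxPileOfClothes is a searchable clothes-pile object that outlines when the player enters its inner sphere and spawns a configurable actor once searched.
; CanInteract, when the status allows searching, disables player input, shows WB_Interact and plays a search montage, sound and fixed timer.
; An Interact press restores input and sets a cancel flag, which the timer checks before marking the pile searched and spawning at the Scene transform.
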(event OnComponentBeginOverlap(InnerSphereCollsion)
  (params (OverlappedComponent :type Primitive%20Component%20Object%20Reference) (OtherActor :type Actor%20Object%20Reference) (OtherComp :type Primitive%20Component%20Object%20Reference) (OtherBodyIndex :type Integer) (bFromSweep :type Boolean) (SweepResult :type Hit%20Result%20Structure%20%28by%20ref%29))
  ;[1 1 1] Inner
  (if (not (Variables|Default|GetSearched?))
    (if (== OtherActor (Game|GetPlayerCharacter 0))
      (Utilities|FlowControl|Sequence
        (:then_0
          (CallFunction|OutlineInneron))))))

(event OnComponentEndOverlap(InnerSphereCollsion)
  (params (OverlappedComponent :type Primitive%20Component%20Object%20Reference) (OtherActor :type Actor%20Object%20Reference) (OtherComp :type Primitive%20Component%20Object%20Reference) (OtherBodyIndex :type Integer))
  ;[1 1 1] Inner
  (if (== OtherActor (Game|GetPlayerCharacter 0))
    (Utilities|FlowControl|Sequence
      (:then_0
        (CallFunction|OutlineInnerOff)))))

(event Custom|show111
  ;[1 1 1] Comment
  (if (Variables|Default|GetCancel?)
    (Variables|Default|SetCancel? false)
    (Widget|RemovefromParent (Variables|Default|GetHoldButtomRef))
    (else
      (Widget|RemovefromParent (Variables|Default|GetHoldButtomRef))
      (Variables|Default|SetSearched? true)
      ;[1 1 1] Comment
      (Utilities|FlowControl|Sequence
        (:then_0
          (CallFunction|OutlineInnerOff)
          (CallFunction|IconLockOff))
        (:then_1
          (Variables|Default|SetBox%20Status "NewEnumerator1"))
        (:then_2
          (CallFunction|SpawKey))))))

(event Custom|Searching
  ;[1 1 1] Searching
  (bind _returnvalue (UserInterface|CreateWidget "/Game/UI/WB_Interact.WB_Interact_C"))
  (bind _output_get (Variables|Default|SetHoldButtomRef _returnvalue))
  (UserInterface|Viewport|AddtoViewport _output_get 0)
  (Input|DisableInput (Variables|Default|GetAs%20BP%20Player) 0))

(event Custom|Spaw%20Key
  (Game|SpawnActorfromClass (Variables|Default|GetClass%20Spaw) (Transformation|GetWorldTransform (Variables|Default|GetScene)) "Undefined" "MultiplyWithRoot" 0 0))

(event Custom|Stop%20Searching
  ;[1 1 1] Comment
  (Widget|RemovefromParent (Variables|Default|GetHoldButtomRef))
  (Input|EnableInput (Variables|Default|GetAs%20BP%20Player) 0)
  (Variables|Default|SetCancel? true))

(event Custom|Icon%20lockOn
  ;[1 1 1] Comment
  (Rendering|SetVisibility (Variables|Default|GetLock%20Icon) true false))

(event Custom|Interact%20Time%20In%20Item
  ;[1 1 1] Comment
  (Utilities|Time|SetTimerbyEvent (delegate Custom|show111) 5.0)
  (Audio|PlaySound2D "/Game/Sounds/Forlay/SFX_Interact_SearchCloth.SFX_Interact_SearchCloth" 1.0 1.0 0.0 0 0))

(event Custom|Icon%20lockOff
  ;[1 1 1] Comment
  (Rendering|SetVisibility (Variables|Default|GetLock%20Icon) false false))

(event Custom|Outline%20innerOn
  ;[1 1 1] Comment
  (Rendering|SetCustomDepthStencilValue (Variables|Default|GetBox_Sprite) 1))

(event Custom|Outline%20innerOff
  ;[1 1 1] Comment
  (Rendering|SetCustomDepthStencilValue (Variables|Default|GetBox_Sprite) 0))

(event EventBeginPlay
  ;[1 1 1] Get player
  (bind _asbp_third_person_character (Utilities|Casting|CastToBP_ThirdPersonCharacter (Game|GetPlayerCharacter 0)))
  (Variables|Default|SetAs%20BP%20Player _asbp_third_person_character))

(event EventCanInteract
  ;[1 1 1] Comment
  (switch Utilities|FlowControl|Switch|SwitchonEN_BoxStatus (Variables|Default|GetBox%20Status)
    (:NewEnumerator0
      (CallFunction|Searching)
      (Animation|Montage|PlayMontage (Variables|/Script/Engine.Character|GetMesh (Variables|Default|GetAs%20BP%20Player)) "/Game/Characters/Character_PP_New/animation/Cha_Search_Montage.Cha_Search_Montage"
        (:then
          (CallFunction|InteractTimeinItem)
          (Class|UserWidget|ListenforInputAction (Variables|Default|GetHoldButtomRef) "Interact" "IE_Pressed" true (delegate Custom|Stop%20Searching)))))))

(fn ConstructionScript
  (Components|Sphere|SetSphereRadius (Variables|Default|GetInnerSphereCollsion) (Variables|Public|GetInnerSphereRadius) true))