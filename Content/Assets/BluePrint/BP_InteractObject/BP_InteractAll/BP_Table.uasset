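; BP_Table is an interactable, optionally locked table that spawns an item, apparently a key, when opened.
; While it is locked, player overlap with the inner sphere toggles a stencil highlight and lock icon.
; CanInteract switches on DoorStatus, searching the player's inventory for LockKey when locked and notifying BP_GameManager of a completed objective on unlock.
; Opening runs through a DoOnce that plays the door sound and spawns the configured class.
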(event OnComponentBeginOverlap(InnerSphereCollsion)
  (params (OverlappedComponent :type Primitive%20Component%20Object%20Reference) (OtherActor :type Actor%20Object%20Reference) (OtherComp :type Primitive%20Component%20Object%20Reference) (OtherBodyIndex :type Integer) (bFromSweep :type Boolean) (SweepResult :type Hit%20Result%20Structure%20%28by%20ref%29))
  ;[1 1 1] Check player overlap
  (if (and (== OtherActor (Game|GetPlayerCharacter 0)) (Variables|Default|GetIt%20Lock?))
    (Rendering|SetCustomDepthStencilValue (Variables|Default|GetBox_Sprite) 1)
    (CallFunction|IconLockon)))

(event OnComponentEndOverlap(InnerSphereCollsion)
  (params (OverlappedComponent :type Primitive%20Component%20Object%20Reference) (OtherActor :type Actor%20Object%20Reference) (OtherComp :type Primitive%20Component%20Object%20Reference) (OtherBodyIndex :type Integer))
  ;[1 1 1] Check player overlap
  (if (and (Variables|Default|GetIt%20Lock?) (== (Game|GetPlayerCharacter 0) OtherActor))
    (Rendering|SetCustomDepthStencilValue (Variables|Default|GetBox_Sprite) 0)
    (CallFunction|IconLockOff)))

(event Custom|Spaw%20Key
  (Game|SpawnActorfromClass (Variables|Default|GetClass%20Spaw) (Math|Transform|MakeTransform (Transformation|GetWorldLocation (Variables|Default|GetScene)) "0, 0, 0" "1.000000,1.000000,1.000000") "Undefined" "MultiplyWithRoot" 0 0))

(event Custom|Icon%20lockOn
  ;[1 1 1] Comment
  (Rendering|SetVisibility (Variables|Default|GetLock%20Icon) true false))

(event Custom|Icon%20lockOff
  ;[1 1 1] Comment
  (Rendering|SetVisibility (Variables|Default|GetLock%20Icon) false false))

(event EventBeginPlay
  ;[1 1 1] Get player
  (bind _asbp_third_person_character (Utilities|Casting|CastToBP_ThirdPersonCharacter (Game|GetPlayerCharacter 0)))
  (Variables|Default|SetAs%20BP%20player _asbp_third_person_character)
  (bind _returnvalue (Actor|GetActorOfClass "/Game/ThirdPerson/Blueprints/BP_Objective/BP_GameManager.BP_GameManager_C"))
  (Variables|Default|SetAs%20Game%20Manager _returnvalue))

(event EventCanInteract
  ;[1 1 1] Comment
  (switch Utilities|FlowControl|Switch|SwitchonEN_DoorStatus (Variables|Default|GetDoorStatus)
    (:NewEnumerator0
      (Variables|Default|SetDoorStatus "NewEnumerator1")
      (Utilities|FlowControl|DoOnce false :!label _label
        (:Completed
          (Audio|PlaySoundatLocation "/Game/Sounds/Forlay/SFX_Interact_DoorOpen.SFX_Interact_DoorOpen" "0, 0, 0" "0, 0, 0" 1.0 1.0 0.0 0 0 0 0)
          (CallFunction|SpawKey))))
    (:NewEnumerator1
      (Variables|Default|SetIt%20Open? true))
    (:NewEnumerator2
      (goto _label))
    (:NewEnumerator3
      (for _array_element (Variables|/Game/ThirdPerson/Blueprints/BPC_Inventory.BPC_Inventory_C|GetInventory (Variables|/Game/ThirdPerson/Blueprints/BP_ThirdPersonCharacter.BP_ThirdPersonCharacter_C|GetBPC_Inventory (Variables|Default|GetAs%20BP%20player)))
        (if (Utilities|Enum|Equal(Enum) _array_element (Variables|Default|GetLockKey))
          (CallFunction|KeyPickUp)
          (Variables|Default|SetIt%20Lock? false)
          (Class|IObjective|CompletedObjective(Message) (Variables|Default|GetAs%20Game%20Manager) 8)
          (goto _label))))))

(fn ConstructionScript)

(fn KeyPickUp
  (switch Utilities|FlowControl|Switch|SwitchonEN_DoorStatus (Variables|Default|GetDoorStatus)
    (:NewEnumerator3
      (Variables|Default|SetDoorStatus "NewEnumerator2")
      (Variables|Default|SetIt%20Lock? false))))