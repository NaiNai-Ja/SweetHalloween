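; Music box key pickup, a sprite that starts transparent until SetKeyopacity reveals it with a sound, stencil highlight and icon.
; Its sphere overlap reports objective 10 to BP_GameManager and, if that objective is current, shows the icon and highlight for the player.
; During objective 11, CanInteract completes the objective and adds the item to the player's inventory.
; After a short delay it destroys itself and shows BP_Candy_3.
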(event OnComponentBeginOverlap(Sphere)
  (params (OverlappedComponent :type Primitive%20Component%20Object%20Reference) (OtherActor :type Actor%20Object%20Reference) (OtherComp :type Primitive%20Component%20Object%20Reference) (OtherBodyIndex :type Integer) (bFromSweep :type Boolean) (SweepResult :type Hit%20Result%20Structure%20%28by%20ref%29))
  (bind _as_game_manager (Variables|Default|GetAs%20Game%20Manager))
  ;[1 1 1] Comment
  (Class|IObjective|CompletedObjective(Message) _as_game_manager 10)
  (if (== (Variables|/Game/ThirdPerson/Blueprints/BP_Objective/BP_GameManager.BP_GameManager_C|GetCurrentObjectiveID _as_game_manager) 10)
    (if (== OtherActor (Game|GetPlayerCharacter 0))
      (CallFunction|IconInneron)
      (Rendering|SetCustomDepthStencilValue (Variables|Default|GetPaperSprite) 1))))

(event OnComponentEndOverlap(Sphere)
  (params (OverlappedComponent :type Primitive%20Component%20Object%20Reference) (OtherActor :type Actor%20Object%20Reference) (OtherComp :type Primitive%20Component%20Object%20Reference) (OtherBodyIndex :type Integer))
  ;[1 1 1] Comment
  (if (== OtherActor (Game|GetPlayerCharacter 0))
    (CallFunction|IconInnerOff)
    (Rendering|SetCustomDepthStencilValue (Variables|Default|GetPaperSprite) 0)))

(event Custom|SetKeyopacity
  (Audio|PlaySoundatLocation "/Game/Sounds/Forlay/SFX_Trigger_PlateDestory.SFX_Trigger_PlateDestory" (Transformation|GetActorLocation) "0, 0, 0" 1.0 1.0 0.0 0 0 0 0)
  (Rendering|SetCustomDepthStencilValue (Variables|Default|GetPaperSprite) 1)
  (Sprite|SetSpriteColor (Variables|Default|GetPaperSprite) "(R=1.000000,G=1.000000,B=1.000000,A=1.000000)")
  (CallFunction|IconInneron))

(event Custom|Icon%20innerOn
  ;[1 1 1] Comment
  (Rendering|SetVisibility (Variables|Default|GetBillboard) true false))

(event Custom|Icon%20innerOff
  ;[1 1 1] Comment
  (Rendering|SetVisibility (Variables|Default|GetBillboard) false false))

(event EventCanInteract
  ;[1 1 1] Comment
  (if (== (Variables|/Game/ThirdPerson/Blueprints/BP_Objective/BP_GameManager.BP_GameManager_C|GetCurrentObjectiveID (Variables|Default|GetAs%20Game%20Manager)) 11)
    (Class|IObjective|CompletedObjective(Message) (Variables|Default|GetAs%20Game%20Manager) 11)
    (Audio|PlaySound2D "/Game/Sounds/Forlay/SFX_GetKey.SFX_GetKey" 1.0 1.0 0.0 0 0)
    (Default|AddItemtoInventory (Variables|/Game/ThirdPerson/Blueprints/BP_ThirdPersonCharacter.BP_ThirdPersonCharacter_C|GetBPC_Inventory (Variables|Default|GetAs%20Player)) (Variables|Default|GetItem))
    (Utilities|FlowControl|Delay 0.2)
    (Utilities|FlowControl|Sequence
      (:then_0
        (Actor|DestroyActor))
      (:then_1
        (bind _returnvalue (Actor|GetActorOfClass "/Game/Assets/BluePrint/BP_Candy_3.BP_Candy_3_C"))
        (Default|Show _returnvalue)))))

(event EventBeginPlay
  ;[1 1 1] Get player BP
  (bind _asbp_third_person_character (Utilities|Casting|CastToBP_ThirdPersonCharacter (Game|GetPlayerCharacter 0)))
  (Variables|Default|SetAs%20Player _asbp_third_person_character)
  (bind _returnvalue (Actor|GetActorOfClass "/Game/ThirdPerson/Blueprints/BP_Objective/BP_GameManager.BP_GameManager_C"))
  (Variables|Default|SetAs%20Game%20Manager _returnvalue)
  (Sprite|SetSpriteColor (Variables|Default|GetPaperSprite) "(R=1.000000,G=1.000000,B=1.000000,A=0.000000)")
  (Rendering|SetVisibility (Variables|Default|GetPaperSprite1) false false))

(fn ConstructionScript)