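; BP_Candy_3 is a hidden candy pickup that serves as the game's ending trigger.
; It starts with a transparent sprite and dark spotlight until the show event reveals both and plays a sound.
; Player overlap with its box reports objective 12 to BP_GameManager, even while hidden.
; If the current objective is then 12, it disables input, displays the WB_Tobecon widget and quits after a delay.
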(event OnComponentBeginOverlap(Box)
  (params (OverlappedComponent :type Primitive%20Component%20Object%20Reference) (OtherActor :type Actor%20Object%20Reference) (OtherComp :type Primitive%20Component%20Object%20Reference) (OtherBodyIndex :type Integer) (bFromSweep :type Boolean) (SweepResult :type Hit%20Result%20Structure%20%28by%20ref%29))
  (bind _as_game_manager (Variables|Default|GetAs%20Game%20Manager))
  ;[1 1 1] Comment
  (if (== OtherActor (Game|GetPlayerCharacter 0))
    (Class|IObjective|CompletedObjective(Message) _as_game_manager 12)
    (if (== (Variables|/Game/ThirdPerson/Blueprints/BP_Objective/BP_GameManager.BP_GameManager_C|GetCurrentObjectiveID _as_game_manager) 12)
      (Input|DisableInput (Game|GetPlayerCharacter 0) (Game|GetPlayerController 0))
      (bind _returnvalue (UserInterface|CreateWidget "/Game/UI/UI_Tak/WB_Tobecon.WB_Tobecon_C"))
      (UserInterface|Viewport|AddtoViewport _returnvalue 0)
      (Utilities|FlowControl|Delay 6.0)
      (Game|QuitGame 0 "Quit" false))))

(event Custom|show
  (Sprite|SetSpriteColor (Variables|Default|GetPaperSprite) "(R=1.000000,G=1.000000,B=1.000000,A=1.000000)")
  (Audio|PlaySoundatLocation "/Game/Sounds/BGM/BGM_Mainmenu1.BGM_Mainmenu1" (Transformation|GetActorLocation) "0, 0, 0" 1.0 1.0 0.0 0 0 0 0)
  (Rendering|Components|Light|SetIntensity (Variables|Default|GetSpotLight) 5e+02))

(event EventBeginPlay
  ;[1 1 1] Get player BP
  (bind _asbp_third_person_character (Utilities|Casting|CastToBP_ThirdPersonCharacter (Game|GetPlayerCharacter 0)))
  (Variables|Default|SetAs%20Player _asbp_third_person_character)
  (bind _returnvalue (Actor|GetActorOfClass "/Game/ThirdPerson/Blueprints/BP_Objective/BP_GameManager.BP_GameManager_C"))
  (Variables|Default|SetAs%20Game%20Manager _returnvalue)
  (Sprite|SetSpriteColor (Variables|Default|GetPaperSprite) "(R=1.000000,G=1.000000,B=1.000000,A=0.000000)")
  (Rendering|Components|Light|SetIntensity (Variables|Default|GetSpotLight) 0.0))

(fn ConstructionScript)