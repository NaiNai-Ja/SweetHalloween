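; BP_Ghost_1 is a ghost actor that plays a crying sound when the player walks into its box while carrying the storage key.
; It caches the third-person player character on BeginPlay.
; On overlap it searches the player's inventory component for the "StorageKey" entry.
; A DoOnce gate then plays the crying sound at its scene location and sets a Ready flag, which nothing in this blueprint reads.
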(event OnComponentBeginOverlap(Box)
  (params (OverlappedComponent :type Primitive%20Component%20Object%20Reference) (OtherActor :type Actor%20Object%20Reference) (OtherComp :type Primitive%20Component%20Object%20Reference) (OtherBodyIndex :type Integer) (bFromSweep :type Boolean) (SweepResult :type Hit%20Result%20Structure%20%28by%20ref%29))
  (if (== OtherActor (Game|GetPlayerCharacter 0))
    (for _array_element (Variables|/Game/ThirdPerson/Blueprints/BPC_Inventory.BPC_Inventory_C|GetInventory (Variables|/Game/ThirdPerson/Blueprints/BP_ThirdPersonCharacter.BP_ThirdPersonCharacter_C|GetBPC_Inventory (Variables|Default|GetAs%20BP%20Player)))
      (if (Utilities|Enum|Equal(Enum) _array_element "StorageKey")
        (Utilities|FlowControl|DoOnce false
          (:Completed
            (Audio|PlaySoundatLocation "/Game/Sounds/Forlay/SFX_Trigger_Ghostcrying.SFX_Trigger_Ghostcrying" (Transformation|GetWorldLocation (Variables|Default|GetScene)) "0, 0, 0" 1.0 1.0 0.0 0 0 0 0)
            (Variables|Default|SetReady? true)))))))

(event EventBeginPlay
  (bind _asbp_third_person_character (Utilities|Casting|CastToBP_ThirdPersonCharacter (Game|GetPlayerCharacter 0)))
  (Variables|Default|SetAs%20BP%20Player _asbp_third_person_character))

(fn ConstructionScript)