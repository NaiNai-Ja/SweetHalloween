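; Hallway door actor that swings open by itself once the game manager's objective ID reaches the required stage.
; Tick watches that ID and, if the door status is Close, fires once: a delay, a sound, then a timeline rotates the gate pivot.
; Until opened, player overlap shows a lock icon and sets the gate's custom-depth stencil.
; KeyPickUp updates the lock state; construction sets the pivot from a clamped angle.
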(event OnComponentBeginOverlap(BoxTrigger)
  (params (OverlappedComponent :type Primitive%20Component%20Object%20Reference) (OtherActor :type Actor%20Object%20Reference) (OtherComp :type Primitive%20Component%20Object%20Reference) (OtherBodyIndex :type Integer) (bFromSweep :type Boolean) (SweepResult :type Hit%20Result%20Structure%20%28by%20ref%29))
  ;[1 1 1] Check player overlap
  (if (not (Variables|Default|GetIt%20Open?))
    (if (== OtherActor (Game|GetPlayerCharacter 0))
      (if (not (Variables|Default|GetIt%20Open?))
        (Rendering|SetCustomDepthStencilValue (Variables|Default|GetSM-Gate-01-02) 1)
        (CallFunction|IconLockon)))))

(event OnComponentEndOverlap(BoxTrigger)
  (params (OverlappedComponent :type Primitive%20Component%20Object%20Reference) (OtherActor :type Actor%20Object%20Reference) (OtherComp :type Primitive%20Component%20Object%20Reference) (OtherBodyIndex :type Integer))
  ;[1 1 1] Check player overlap
  (if (== (Game|GetPlayerCharacter 0) OtherActor)
    (Rendering|SetCustomDepthStencilValue (Variables|Default|GetSM-Gate-01-02) 0)
    (CallFunction|IconLockOff)))

(event Custom|Door%20Open
  ;[1 1 1] Animation Open
  (bind _door_open (Timeline|Door%20Open%20Anim Play)
    (:Update
      (Transformation|SetRelativeRotation (Variables|Default|GetGatePivot) (Math|Rotator|MakeRotator 0.0 0.0 (Math|Float|Lerp 0.0 1.2e+02 _door_open)) false false))))

(event Custom|Icon%20lockOn
  ;[1 1 1] Comment
  (Rendering|SetVisibility (Variables|Default|GetLock%20Icon) true false))

(event Custom|Icon%20lockOff
  ;[1 1 1] Comment
  (Rendering|SetVisibility (Variables|Default|GetLock%20Icon) false false))

(event EventBeginPlay
  ;[1 1 1] Get player
  (bind _asbp_third_person_character (Utilities|Casting|CastToBP_ThirdPersonCharacter (Game|GetPlayerCharacter 0)))
  (Variables|Default|SetAs%20BP%20player _asbp_third_person_character)
  (bind _returnvalue (Actor|GetActorOfClass "/Game/ThirdPerson/Blueprints/BP_Objective/BP_GameManager.BP_GameManager_C"))
  (Variables|Default|SetAs%20Game%20Manager _returnvalue)
  (CallFunction|IconLockOff))

(event EventTick
  (params (DeltaSeconds :type Float%20%28single-precision%29))
  ;[1 1 1] Comment
  (if (>= (Variables|/Game/ThirdPerson/Blueprints/BP_Objective/BP_GameManager.BP_GameManager_C|GetCurrentObjectiveID (Variables|Default|GetAs%20Game%20Manager)) 2)
    (switch Utilities|FlowControl|Switch|SwitchonEN_DoorStatus (Variables|Default|GetDoorStatus)
      (:NewEnumerator0
        (Utilities|FlowControl|DoOnce false
          (:Completed
            (Utilities|FlowControl|Delay 3.0)
            (Audio|PlaySoundatLocation "/Game/Sounds/Forlay/SFX_Trigger_DoorOpenSlowly.SFX_Trigger_DoorOpenSlowly" (Transformation|GetActorLocation) "0, 0, 0" 5.0 1.0 0.0 "/Game/Sounds/BP_sounds/Ghost_SoundAttenuation.Ghost_SoundAttenuation" 0 0 0)
            (CallFunction|DoorOpen)
            (CallFunction|IconLockOff)
            (Rendering|SetCustomDepthStencilValue (Variables|Default|GetSM-Gate-01-02) 0)
            (Variables|Default|SetIt%20Open? true)))))))

(event EventCanInteract)

(fn ConstructionScript
  (Transformation|SetRelativeRotation (Variables|Default|GetGatePivot) (Math|Rotator|MakeRotator 0.0 0.0 (* (Math|Float|Clamp(Float) (Variables|Default|GetDoor%20Open%20Angle) 0.0 1.2e+02) -1.0)) false false))

(fn KeyPickUp
  (switch Utilities|FlowControl|Switch|SwitchonEN_DoorStatus (Variables|Default|GetDoorStatus)
    (:NewEnumerator3
      (Variables|Default|SetDoorStatus "NewEnumerator2")
      (Variables|Default|SetIt%20Lock? false))))