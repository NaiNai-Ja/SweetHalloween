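; BP_SpawnerCrowbar is a trigger actor that drops a crowbar into the level during a specific objective.
; On BeginPlay it caches the BP_GameManager, and Box1 arms the spawner when the player character overlaps it while the matching objective is current.
; Once armed, the first overlap on Box by any actor plays a drop sound and spawns BP_Crowbar at the Arrow's location, guarded by DoOnce.
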(event OnComponentBeginOverlap(Box1)
  (params (OverlappedComponent :type Primitive%20Component%20Object%20Reference) (OtherActor :type Actor%20Object%20Reference) (OtherComp :type Primitive%20Component%20Object%20Reference) (OtherBodyIndex :type Integer) (bFromSweep :type Boolean) (SweepResult :type Hit%20Result%20Structure%20%28by%20ref%29))
  (Utilities|Casting|CastToBP_ThirdPersonCharacter OtherActor)
  (if (== (Variables|/Game/ThirdPerson/Blueprints/BP_Objective/BP_GameManager.BP_GameManager_C|GetCurrentObjectiveID (Variables|Default|GetAs%20Game%20Manager)) 6)
    (Variables|Default|SetsetBool true)))

(event OnComponentBeginOverlap(Box)
  (params (OverlappedComponent :type Primitive%20Component%20Object%20Reference) (OtherActor :type Actor%20Object%20Reference) (OtherComp :type Primitive%20Component%20Object%20Reference) (OtherBodyIndex :type Integer) (bFromSweep :type Boolean) (SweepResult :type Hit%20Result%20Structure%20%28by%20ref%29))
  (bind _arrow (Variables|Default|GetArrow))
  (bind _returnvalue (Transformation|GetWorldLocation _arrow))
  (if (Variables|Default|GetsetBool)
    (Utilities|FlowControl|DoOnce false
      (:Completed
        (Audio|PlaySoundatLocation "/Game/Sounds/Forlay/SFX_Trigger_CrowbarDrop.SFX_Trigger_CrowbarDrop" _returnvalue "0, 0, 0" 1.0 1.0 0.0 0 0 0 0)
        (Game|SpawnActorfromClass "/Game/Assets/BluePrint/Door/BP_KeyAll/BP_Crowbar.BP_Crowbar_C" (Math|Transform|MakeTransform _returnvalue "0, 0, 0" "1.000000,1.000000,1.000000") "Undefined" "MultiplyWithRoot" 0 0)))))

(event EventBeginPlay
  (bind _returnvalue (Actor|GetActorOfClass "/Game/ThirdPerson/Blueprints/BP_Objective/BP_GameManager.BP_GameManager_C"))
  (Variables|Default|SetAs%20Game%20Manager _returnvalue))

(fn ConstructionScript)