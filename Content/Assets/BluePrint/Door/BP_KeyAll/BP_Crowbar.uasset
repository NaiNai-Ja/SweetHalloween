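; BP_Crowbar is a crowbar pickup that adds its item to the player's inventory component when interacted with, plays a pickup sound and destroys itself after a short delay.
; Its paper sprite bobs endlessly through two timelines, one played forward and one in reverse, that retrigger each other.
; A sphere overlap with the player shows an interact icon and sets the sprite's custom depth stencil value, reverting both on exit.
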(event OnComponentBeginOverlap(Sphere)
  (params (OverlappedComponent :type Primitive%20Component%20Object%20Reference) (OtherActor :type Actor%20Object%20Reference) (OtherComp :type Primitive%20Component%20Object%20Reference) (OtherBodyIndex :type Integer) (bFromSweep :type Boolean) (SweepResult :type Hit%20Result%20Structure%20%28by%20ref%29))
  ;[1 1 1] Comment
  (if (== OtherActor (Game|GetPlayerCharacter 0))
    (CallFunction|IconInneron)
    (Rendering|SetCustomDepthStencilValue (Variables|Default|GetPaperSprite) 1)))

(event OnComponentEndOverlap(Sphere)
  (params (OverlappedComponent :type Primitive%20Component%20Object%20Reference) (OtherActor :type Actor%20Object%20Reference) (OtherComp :type Primitive%20Component%20Object%20Reference) (OtherBodyIndex :type Integer))
  ;[1 1 1] Comment
  (if (== OtherActor (Game|GetPlayerCharacter 0))
    (CallFunction|IconInnerOff)
    (Rendering|SetCustomDepthStencilValue (Variables|Default|GetPaperSprite) 0)))

(event Custom|PlayAni
  ;[1 1 1] Floating
  (bind _z_movemant (Timeline|Timeline PlayFromStart)
    (:Update
      (Transformation|SetRelativeLocation (Variables|Default|GetPaperSprite) _z_movemant false false))
    (:Finished
      (CallFunction|PlayReverse))))

(event Custom|Icon%20innerOn
  ;[1 1 1] Comment
  (Rendering|SetVisibility (Variables|Default|GetinnerInteractIcon) true false))

(event Custom|Icon%20innerOff
  ;[1 1 1] Comment
  (Rendering|SetVisibility (Variables|Default|GetinnerInteractIcon) false false))

(event Custom|PlayReverse
  ;[1 1 1] Floating
  (bind _z_movemant (Timeline|Timeline_0 ReverseFromEnd)
    (:Update
      (Transformation|SetRelativeLocation (Variables|Default|GetPaperSprite) _z_movemant false false))
    (:Finished
      (CallFunction|PlayAni))))

(event EventCanInteract
  ;[1 1 1] Comment
  (Audio|PlaySound2D "/Game/Sounds/Forlay/SFX_GetKey.SFX_GetKey" 1.0 1.0 0.0 0 0)
  (Default|AddItemtoInventory (Variables|/Game/ThirdPerson/Blueprints/BP_ThirdPersonCharacter.BP_ThirdPersonCharacter_C|GetBPC_Inventory (Variables|Default|GetAs%20Player)) (Variables|Default|GetItem))
  (Utilities|FlowControl|Delay 0.2)
  (Actor|DestroyActor))

(event EventBeginPlay
  ;[1 1 1] Get player BP
  (bind _asbp_third_person_character (Utilities|Casting|CastToBP_ThirdPersonCharacter (Game|GetPlayerCharacter 0)))
  (Variables|Default|SetAs%20Player _asbp_third_person_character)
  (CallFunction|PlayAni))

(fn ConstructionScript)