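; Ghost kid character that walks along an array of target points, then fades away and disappears.
; After a short delay on BeginPlay, MoveToPoint uses AI MoveTo toward the current point, incrementing the index and calling itself on each success.
; At index 1, a timeline runs alongside the movement, lerping opacity to zero through the MPC_InvisKid parameter collection, then destroys the actor.
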(event Custom|Move%20to%20point
  ;[1 1 1] MovetoPlayer
  (if (== (Variables|Default|GettoPoint) 1)
    (Utilities|FlowControl|Sequence
      (:then_0
        (bind _door_open (Timeline|Timeline Play)
          (:Update
            (Rendering|Material|SetScalarParameterValue "/Game/Characters/BP_KidGhost/Ghost_Guide/MPC_InvisKid.MPC_InvisKid" "Mash Opacity" (Math|Float|Lerp 1.0 0.0 _door_open) :!class /Script/Engine.KismetMaterialLibrary))
          (:Finished
            (Actor|DestroyActor))))
      (:then_1
        (AI|AIMoveTo self (Transformation|GetActorLocation (Utilities|Array|Get(acopy) (Variables|Default|GetPoint) (Variables|Default|GettoPoint))) (Utilities|Array|Get(acopy) (Variables|Default|GetPoint) (Variables|Default|GettoPoint)) 5.0 false :!label _label
          (:OnSuccess
            (Variables|Default|SettoPoint (+ (Variables|Default|GettoPoint) 1))
            (Utilities|FlowControl|Delay 0.5)
            (CallFunction|MovetoPoint)))))
    (else
      (goto _label))))

(event EventBeginPlay
  ;[1 1 1] Get EndPoint
  (Variables|Default|SettoPoint 0)
  (Utilities|FlowControl|Delay 1.5)
  (CallFunction|MovetoPoint))

(fn ConstructionScript)