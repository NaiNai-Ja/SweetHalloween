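; Ghost enemy that hunts the player at low sanity, triggering game over and pausing on capsule hit at that level.
; Tick copies PlayerMind into a RepNotify, which sets blackboard keys and teleports the ghost to a fixed spot unless sanity is low and Hunt is set.
; "PlayerSane?" is true when sanity is low, despite its name.
; A sphere overlap fades opacity through a timeline-driven material parameter collection and updates the player-distance key.
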(event OnComponentHit(CapsuleComponent)
  (params (HitComponent :type Primitive%20Component%20Object%20Reference) (OtherActor :type Actor%20Object%20Reference) (OtherComp :type Primitive%20Component%20Object%20Reference) (NormalImpulse :type Vector :default "0, 0, 0") (Hit :type Hit%20Result%20Structure%20%28by%20ref%29))
  (if (== OtherActor (Variables|Default|GetAs%20BP_Player))
    (if (<= (Variables|Default|GetGetPlayermind) 0.3)
      (Input|DisableInput (Variables|Default|GetAs%20BP_Player) (Game|GetPlayerController 0))
      (bind _returnvalue (UserInterface|CreateWidget "/Game/UI/UI_Tak/WB_Gameover.WB_Gameover_C"))
      (UserInterface|Viewport|AddtoViewport _returnvalue 0)
      (Game|SetGamePaused true))))

(event OnComponentBeginOverlap(Sphere)
  (params (OverlappedComponent :type Primitive%20Component%20Object%20Reference) (OtherActor :type Actor%20Object%20Reference) (OtherComp :type Primitive%20Component%20Object%20Reference) (OtherBodyIndex :type Integer) (bFromSweep :type Boolean) (SweepResult :type Hit%20Result%20Structure%20%28by%20ref%29))
  (if (== OtherActor (Variables|Default|GetAs%20BP_Player))
    (CallFunction|ShowItself)
    (AI|Components|Blackboard|SetValueasBool (AI|GetBlackboard (AI|GetAIController self)) (Utilities|Name|MakeLiteralName "PlayerIsToFar?") false)))

(event OnComponentEndOverlap(Sphere)
  (params (OverlappedComponent :type Primitive%20Component%20Object%20Reference) (OtherActor :type Actor%20Object%20Reference) (OtherComp :type Primitive%20Component%20Object%20Reference) (OtherBodyIndex :type Integer))
  (if (== OtherActor (Variables|Default|GetAs%20BP_Player))
    (CallFunction|HideItSelf)
    (AI|Components|Blackboard|SetValueasBool (AI|GetBlackboard (AI|GetAIController self)) (Utilities|Name|MakeLiteralName "PlayerIsToFar?") true)))

(event Custom|Hide%20it%20self
  (bind _showandhide (Timeline|Timeline Reverse)
    (:Update
      (Rendering|Material|SetScalarParameterValue "/Game/Characters/BP_Enemy_01/Model_Enemy_1/MPC_Enemy_01.MPC_Enemy_01" "Mash Opacity" (Math|Float|Lerp 0.0 1.0 _showandhide) :!class /Script/Engine.KismetMaterialLibrary))))

(event Custom|ShowItself
  (bind _showandhide (Timeline|Timeline Play)
    (:Update
      (Rendering|Material|SetScalarParameterValue "/Game/Characters/BP_Enemy_01/Model_Enemy_1/MPC_Enemy_01.MPC_Enemy_01" "Mash Opacity" (Math|Float|Lerp 0.0 1.0 _showandhide) :!class /Script/Engine.KismetMaterialLibrary))))

(event EventTick
  (params (DeltaSeconds :type Float%20%28single-precision%29))
  (Utilities|FlowControl|Sequence
    (:then_0
      (Variables|Default|SetGetPlayermind (Variables|/Game/ThirdPerson/Blueprints/BPC_PlayerStatus.BPC_PlayerStatus_C|GetPlayer%20Mind (Variables|/Game/ThirdPerson/Blueprints/BP_ThirdPersonCharacter.BP_ThirdPersonCharacter_C|GetBPC_PlayerStatus (Variables|Default|GetAs%20BP_Player))))
      (if (Variables|Default|GetCanHunt)
        (Variables|Default|SetHunt true)))))

(event EventBeginPlay
  (bind _asbp_third_person_character (Utilities|Casting|CastToBP_ThirdPersonCharacter (Game|GetPlayerCharacter 0)))
  (bind _output_get (Variables|Default|SetAs%20BP_Player _asbp_third_person_character))
  (Variables|Default|SetGetPlayermind (Variables|/Game/ThirdPerson/Blueprints/BPC_PlayerStatus.BPC_PlayerStatus_C|GetPlayer%20Mind (Variables|/Game/ThirdPerson/Blueprints/BP_ThirdPersonCharacter.BP_ThirdPersonCharacter_C|GetBPC_PlayerStatus _output_get)))
  (CallFunction|HideItSelf)
  (bind _returnvalue (Actor|GetActorOfClass "/Game/ThirdPerson/Blueprints/BP_Objective/BP_GameManager.BP_GameManager_C"))
  (Variables|Default|SetAs%20Game%20Manager _returnvalue)
  (bind _returnvalue_2 (Actor|GetActorOfClass "/Game/Characters/BP_Enemy_01/AI_BP_01/Enemy_controller_01.Enemy_controller_01_C"))
  (Variables|Default|SetAi%20contraller _returnvalue_2)
  (Audio|SpawnSoundAttached "/Game/Sounds/Ghost_SFX/SFX_GhostBL_CloseUpSound.SFX_GhostBL_CloseUpSound" (Variables|Character|GetMesh) "None" "0, 0, 0" "0, 0, 0" "KeepRelativeOffset" false 1.0 1.0 0.0 0 0))

(fn ConstructionScript)

(fn OnRepGetPlayermind
  (bind _returnvalue (Utilities|Name|MakeLiteralName "PlayerSane?"))
  (bind _self self)
  (bind _returnvalue_2 (AI|GetAIController _self))
  (bind _returnvalue_3 (AI|GetBlackboard _returnvalue_2))
  (if (<= (Variables|Default|GetGetPlayermind) 0.3)
    (if (Variables|Default|GetHunt)
      (AI|Components|Blackboard|SetValueasBool _returnvalue_3 _returnvalue true)
      (else
        (AI|Components|Blackboard|SetValueasBool _returnvalue_3 _returnvalue false :!label _label)
        (AI|Components|Blackboard|SetValueasBool _returnvalue_3 (Utilities|Name|MakeLiteralName "PlayerIsToFar?") true)
        (Transformation|SetActorRelativeLocation "-2310.000000,4850.000000,190.000000" false true)))
    (else
      (goto _label))))