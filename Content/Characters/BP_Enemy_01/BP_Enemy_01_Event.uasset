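; Enemy 01 event actor that stages a ghost effect with a flickering spotlight.
; BeginPlay hides the ghost by zeroing "Mash Opacity" in MPC_Enemy_01.
; Event_ghost tints the light warm, then a self-looping randomized delay and FlipFlop alternate dim light at zero opacity with bright light at full opacity.
; DestroySelf removes the actor, while the FlickeringLight graph is empty.
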(event Custom|DestroySelf
  (Actor|DestroyActor))

(event Custom|Event_ghost
  (bind _spotlight (Variables|Default|GetSpotLight))
  (Rendering|Components|Light|SetLightColor (Variables|Default|GetSpotLight) "(R=1.000000,G=0.643137,B=0.317647,A=1.000000)" true)
  (Utilities|FlowControl|RetriggerableDelay (Math|Random|RandomFloatinRange (Variables|Default|GetMinTime) (Variables|Default|GetMaxTime)) :!label _label)
  (Utilities|FlowControl|FlipFlop
    (:A
      (Rendering|Components|Light|SetIntensity _spotlight 1.0)
      (Rendering|Material|SetScalarParameterValue "/Game/Characters/BP_Enemy_01/Model_Enemy_1/MPC_Enemy_01.MPC_Enemy_01" "Mash Opacity" 0.0 :!class /Script/Engine.KismetMaterialLibrary)
      (goto _label))
    (:B
      (Rendering|Components|Light|SetIntensity _spotlight 5e+01)
      (Rendering|Material|SetScalarParameterValue "/Game/Characters/BP_Enemy_01/Model_Enemy_1/MPC_Enemy_01.MPC_Enemy_01" "Mash Opacity" 1.0 :!class /Script/Engine.KismetMaterialLibrary)
      (goto _label))))

(event EventBeginPlay
  (Rendering|Material|SetScalarParameterValue "/Game/Characters/BP_Enemy_01/Model_Enemy_1/MPC_Enemy_01.MPC_Enemy_01" "Mash Opacity" 0.0 :!class /Script/Engine.KismetMaterialLibrary))

(fn ConstructionScript)

(fn FlickeringLight)