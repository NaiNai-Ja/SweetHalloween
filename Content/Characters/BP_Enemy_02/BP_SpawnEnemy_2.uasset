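; BP_SpawnEnemy_2 is a placed marker actor that supplies four world locations to the controller for the second enemy type.
; On BeginPlay it gathers the world locations of its four Arrow components into the SpawnEnemy2 array.
; It then finds an Enemy_controller_02 with GetActorOfClass and copies that array into its NewLocation variable.
; The Blueprint itself spawns nothing.
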(event EventBeginPlay
  (bind _output_get (Variables|Default|SetSpawnEnemy_2 (Utilities|Array|MakeArray (Transformation|GetWorldLocation (Variables|Default|GetArrow1)) (Transformation|GetWorldLocation (Variables|Default|GetArrow2)) (Transformation|GetWorldLocation (Variables|Default|GetArrow3)) (Transformation|GetWorldLocation (Variables|Default|GetArrow4)))))
  (bind _returnvalue (Actor|GetActorOfClass "/Game/Characters/BP_Enemy_02/AI_BP_02/Enemy_controller_02.Enemy_controller_02_C"))
  (Variables|/Game/Characters/BP_Enemy_02/AI_BP_02/Enemy_controller_02.Enemy_controller_02_C|SetNewLocation _returnvalue _output_get))

(fn ConstructionScript)