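; BP_Enemy_02 is an enemy that drains the player's PlayerMind on capsule hits and changes opacity with that value.
; It copies PlayerMind from BPCPlayerStatus every Tick into a RepNotify variable, whose OnRep sets "Mash Opacity" in MPC_Enemy_02 to one minus that value.
; Tick also polls BP_GameManager and teleports the enemy once to a hard-coded location when CurrentObjectiveID is 2.
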(event OnComponentHit(CapsuleComponent)
  (params (HitComponent :type Primitive%20Component%20Object%20Reference) (OtherActor :type Actor%20Object%20Reference) (OtherComp :type Primitive%20Component%20Object%20Reference) (NormalImpulse :type Vector :default "0, 0, 0") (Hit :type Hit%20Result%20Structure%20%28by%20ref%29))
  (bind _as_bp_player (Variables|Default|GetAs%20BP_Player))
  (bind _bpc_playerstatus (Variables|/Game/ThirdPerson/Blueprints/BP_ThirdPersonCharacter.BP_ThirdPersonCharacter_C|GetBPC_PlayerStatus _as_bp_player))
  (if (== OtherActor _as_bp_player)
    (Variables|/Game/ThirdPerson/Blueprints/BPC_PlayerStatus.BPC_PlayerStatus_C|SetPlayer%20Mind _bpc_playerstatus (- (Variables|/Game/ThirdPerson/Blueprints/BPC_PlayerStatus.BPC_PlayerStatus_C|GetPlayer%20Mind _bpc_playerstatus) 0.1))))

(event EventTick
  (params (DeltaSeconds :type Float%20%28single-precision%29))
  (Variables|Default|SetGetPlayermind (Variables|/Game/ThirdPerson/Blueprints/BPC_PlayerStatus.BPC_PlayerStatus_C|GetPlayer%20Mind (Variables|/Game/ThirdPerson/Blueprints/BP_ThirdPersonCharacter.BP_ThirdPersonCharacter_C|GetBPC_PlayerStatus (Variables|Default|GetAs%20BP_Player))))
  (if (== (Variables|/Game/ThirdPerson/Blueprints/BP_Objective/BP_GameManager.BP_GameManager_C|GetCurrentObjectiveID (Variables|Default|GetNewVar)) 2)
    (Utilities|FlowControl|DoOnce false
      (:Completed
        (Transformation|SetActorLocation "660.000000,2430.000000,70.000000" false false)))))

(event EventBeginPlay
  (bind _asbp_third_person_character (Utilities|Casting|CastToBP_ThirdPersonCharacter (Game|GetPlayerCharacter 0)))
  (bind _output_get (Variables|Default|SetAs%20BP_Player _asbp_third_person_character))
  (Variables|Default|SetGetPlayermind (Variables|/Game/ThirdPerson/Blueprints/BPC_PlayerStatus.BPC_PlayerStatus_C|GetPlayer%20Mind (Variables|/Game/ThirdPerson/Blueprints/BP_ThirdPersonCharacter.BP_ThirdPersonCharacter_C|GetBPC_PlayerStatus _output_get)))
  (bind _returnvalue (Actor|GetActorOfClass "/Game/ThirdPerson/Blueprints/BP_Objective/BP_GameManager.BP_GameManager_C"))
  (Variables|Default|SetNewVar _returnvalue))

(fn ConstructionScript)

(fn OnRepGetPlayermind
  (Rendering|Material|SetScalarParameterValue "/Game/Characters/BP_Enemy_02/Model_Enemy_2/MPC_Enemy_02.MPC_Enemy_02" "Mash Opacity" (- 1.0 (Variables|Default|GetGetPlayermind)) :!class /Script/Engine.KismetMaterialLibrary))