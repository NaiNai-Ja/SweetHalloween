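; BP-Gate-01 is a dungeon gate that swings open on a timeline when OpenDoorCheck is triggered, guarded by a DoOnce.
; A box trigger toggles the mesh's custom stencil value and sets the player character's InteractWith while the player overlaps.
; The construction script previews a clamped, negated DoorOpenAngle on the pivot, opposite in sign to the animation.
; Item-count check and sound nodes are left unconnected.
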(event OnComponentBeginOverlap(BoxTrigger)
  (params (OverlappedComponent :type Primitive%20Component%20Object%20Reference) (OtherActor :type Actor%20Object%20Reference) (OtherComp :type Primitive%20Component%20Object%20Reference) (OtherBodyIndex :type Integer) (bFromSweep :type Boolean) (SweepResult :type Hit%20Result%20Structure%20%28by%20ref%29))
  ;[1 1 1] Check player overlap
  (if (== OtherActor (Variables|Default|GetAs%20BP%20Third%20Person%20Character))
    (Rendering|SetCustomDepthStencilValue (Variables|Default|GetSM-Gate-01-01) 1)
    (Variables|/Game/ThirdPerson/Blueprints/BP_ThirdPersonCharacter.BP_ThirdPersonCharacter_C|Setinteract%20with (Variables|Default|GetAs%20BP%20Third%20Person%20Character) 1.0)))

(event OnComponentEndOverlap(BoxTrigger)
  (params (OverlappedComponent :type Primitive%20Component%20Object%20Reference) (OtherActor :type Actor%20Object%20Reference) (OtherComp :type Primitive%20Component%20Object%20Reference) (OtherBodyIndex :type Integer))
  ;[1 1 1] Check player overlap
  (if (== (Variables|Default|GetAs%20BP%20Third%20Person%20Character) OtherActor)
    (Rendering|SetCustomDepthStencilValue (Variables|Default|GetSM-Gate-01-01) 0)
    (Variables|/Game/ThirdPerson/Blueprints/BP_ThirdPersonCharacter.BP_ThirdPersonCharacter_C|Setinteract%20with (Variables|Default|GetAs%20BP%20Third%20Person%20Character) 0.0)))

(event Custom|Door%20Open
  ;[1 1 1] Animation Open
  (bind _door_open (Timeline|Door%20Open%20Anim Play)
    (:Update
      (Transformation|SetRelativeRotation (Variables|Default|GetGatePivot) (Math|Rotator|MakeRotator 0.0 0.0 (Math|Float|Lerp 0.0 1.2e+02 _door_open)) false false))))

(event Custom|Open%20Door%20Check
  ;[1 1 1] Check condition
  (Utilities|FlowControl|DoOnce false
    (:Completed
      (CallFunction|DoorOpen))))

(event EventBeginPlay
  ;[1 1 1] Get player
  (bind _asbp_third_person_character (Utilities|Casting|CastToBP_ThirdPersonCharacter (Game|GetPlayerCharacter 0)))
  (Variables|Default|SetAs%20BP%20Third%20Person%20Character _asbp_third_person_character))

(fn ConstructionScript
  (Transformation|SetRelativeRotation (Variables|Default|GetGatePivot) (Math|Rotator|MakeRotator 0.0 0.0 (* (Math|Float|Clamp(Float) (Variables|Default|GetDoor%20Open%20Angle) 0.0 1.2e+02) -1.0)) false false))