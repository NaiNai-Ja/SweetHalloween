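; BP_TeaTable is an interactable tea table that calls sanity regeneration on the player and reports an objective as completed.
; Overlapping its inner sphere, sized in the Construction Script, toggles a custom depth stencil highlight and an interact icon for the player only.
; CanInteract calls RegenSenity on the player's status component each time, while a DoOnce limits the BP_GameManager objective message to the first use.
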(event OnComponentBeginOverlap(InnerSphereCollsion)
  (params (OverlappedComponent :type Primitive%20Component%20Object%20Reference) (OtherActor :type Actor%20Object%20Reference) (OtherComp :type Primitive%20Component%20Object%20Reference) (OtherBodyIndex :type Integer) (bFromSweep :type Boolean) (SweepResult :type Hit%20Result%20Structure%20%28by%20ref%29))
  ;[1 1 1] Inner
  (if (== OtherActor (Game|GetPlayerCharacter 0))
    (Utilities|FlowControl|Sequence
      (:then_0
        (Rendering|SetCustomDepthStencilValue (Variables|Default|GetStaticMesh) 1))
      (:then_1
        (Rendering|SetVisibility (Variables|Default|GetinnerInteractIcon) true false)))))

(event OnComponentEndOverlap(InnerSphereCollsion)
  (params (OverlappedComponent :type Primitive%20Component%20Object%20Reference) (OtherActor :type Actor%20Object%20Reference) (OtherComp :type Primitive%20Component%20Object%20Reference) (OtherBodyIndex :type Integer))
  ;[1 1 1] Inner
  (if (== OtherActor (Game|GetPlayerCharacter 0))
    (Utilities|FlowControl|Sequence
      (:then_0
        (Rendering|SetCustomDepthStencilValue (Variables|Default|GetStaticMesh) 0))
      (:then_1
        (Rendering|SetVisibility (Variables|Default|GetinnerInteractIcon) false false)))))

(event EventBeginPlay
  ;[1 1 1] Get player
  (bind _asbp_third_person_character (Utilities|Casting|CastToBP_ThirdPersonCharacter (Game|GetPlayerCharacter 0)))
  (Variables|Default|SetAs%20BP%20Third%20Person%20Character _asbp_third_person_character)
  (bind _returnvalue (Actor|GetActorOfClass "/Game/ThirdPerson/Blueprints/BP_Objective/BP_GameManager.BP_GameManager_C"))
  (Variables|Default|SetAs%20Game%20Manager _returnvalue))

(event EventCanInteract
  (Default|RegenSenity (Variables|/Game/ThirdPerson/Blueprints/BP_ThirdPersonCharacter.BP_ThirdPersonCharacter_C|GetBPC_PlayerStatus (Variables|Default|GetAs%20BP%20Third%20Person%20Character)))
  (Utilities|FlowControl|DoOnce false
    (:Completed
      (Class|IObjective|CompletedObjective(Message) (Variables|Default|GetAs%20Game%20Manager)))))

(fn ConstructionScript
  (Components|Sphere|SetSphereRadius (Variables|Default|GetInnerSphereCollsion) (Variables|Public|GetInnerSphereRadius) true))