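; Storage door actor that the player opens by interacting, optionally requiring a key from their inventory.
; Box overlap toggles a custom-depth highlight and, if locked, a lock icon.
; CanInteract switches on door status, checks inventory for LockKey, then once notifies the game manager's objective, plays a sound and snaps the pivot open, bypassing the DoorOpen timeline.
; The construction script sets the initial angle from clamped DoorOpenAngle.
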(event OnComponentBeginOverlap(BoxTrigger)
  (params (OverlappedComponent :type Primitive%20Component%20Object%20Reference) (OtherActor :type Actor%20Object%20Reference) (OtherComp :type Primitive%20Component%20Object%20Reference) (OtherBodyIndex :type Integer) (bFromSweep :type Boolean) (SweepResult :type Hit%20Result%20Structure%20%28by%20ref%29))
  ;[1 1 1] Check player overlap
  (if (not (Variables|Default|GetIt%20Open?))
    (if (== OtherActor (Game|GetPlayerCharacter 0))
      (if (not (Variables|Default|GetIt%20Open?))
        (Rendering|SetCustomDepthStencilValue (Variables|Default|GetSM-Gate-01-02) 1)
        (if (Variables|Default|GetIt%20Lock?)
          (CallFunction|IconLockon))))))

(event OnComponentEndOverlap(BoxTrigger)
  (params (OverlappedComponent :type Primitive%20Component%20Object%20Reference) (OtherActor :type Actor%20Object%20Reference) (OtherComp :type Primitive%20Component%20Object%20Reference) (OtherBodyIndex :type Integer))
  ;[1 1 1] Check player overlap
  (if (== (Game|GetPlayerCharacter 0) OtherActor)
    (Rendering|SetCustomDepthStencilValue (Variables|Default|GetSM-Gate-01-02) 0)
    (if (Variables|Default|GetIt%20Lock?)
      (CallFunction|IconLockOff))))

(event Custom|Door%20Open
  ;[1 1 1] Animation Open
  (bind _door_open (Timeline|Door%20Open%20Anim Play)
    (:Update
      (Transformation|SetRelativeRotation (Variables|Default|GetGatePivot) (Math|Rotator|MakeRotator 0.0 0.0 1.2e+02) false false))))

(event Custom|Icon%20lockOn
  ;[1 1 1] Comment
  (Rendering|SetVisibility (Variables|Default|GetLock%20Icon) true false))

(event Custom|Icon%20lockOff
  ;[1 1 1] Comment
  (Rendering|SetVisibility (Variables|Default|GetLock%20Icon) false false))

(event EventBeginPlay
  ;[1 1 1] Get player
  (bind _asbp_third_person_character (Utilities|Casting|CastToBP_ThirdPersonCharacter (Game|GetPlayerCharacter 0)))
  (Variables|Default|SetAs%20BP%20player _asbp_third_person_character)
  (Rendering|SetVisibility (Variables|Default|GetLock%20Icon) false false)
  (bind _returnvalue (Actor|GetActorOfClass "/Game/ThirdPerson/Blueprints/BP_Objective/BP_GameManager.BP_GameManager_C"))
  (Variables|Default|SetAs%20GameManager _returnvalue))

(event EventCanInteract
  ;[1 1 1] Comment
  (switch Utilities|FlowControl|Switch|SwitchonEN_DoorStatus (Variables|Default|GetDoorStatus)
    (:NewEnumerator0
      (Variables|Default|SetDoorStatus "NewEnumerator1")
      (CallFunction|IconLockOff)
      (Class|IObjective|CompletedObjective(Message) (Variables|Default|GetAs%20GameManager) 3 :!label _label)
      (Utilities|FlowControl|DoOnce false
        (:Completed
          (Audio|PlaySoundatLocation "/Game/Sounds/Forlay/SFX_Interact_DoorOpen.SFX_Interact_DoorOpen" (Transformation|GetActorLocation) "0, 0, 0" 1.0 1.0 0.0 0 0 0 0)
          (Transformation|SetRelativeRotation (Variables|Default|GetGatePivot) (Math|Rotator|MakeRotator 0.0 0.0 1.2e+02) false false)
          (Rendering|SetCustomDepthStencilValue (Variables|Default|GetSM-Gate-01-02) 0))))
    (:NewEnumerator1
      (Variables|Default|SetIt%20Open? true))
    (:NewEnumerator2
      (goto _label))
    (:NewEnumerator3
      (for _array_element (Variables|/Game/ThirdPerson/Blueprints/BPC_Inventory.BPC_Inventory_C|GetInventory (Variables|/Game/ThirdPerson/Blueprints/BP_ThirdPersonCharacter.BP_ThirdPersonCharacter_C|GetBPC_Inventory (Variables|Default|GetAs%20BP%20player)))
        (if (Utilities|Enum|Equal(Enum) _array_element (Variables|Default|GetLock%20Key))
          (CallFunction|KeyPickUp)
          (Variables|Default|SetIt%20Open? true)
          (CallFunction|IconLockOff)
          (goto _label))))))

(fn ConstructionScript
  (Transformation|SetRelativeRotation (Variables|Default|GetGatePivot) (Math|Rotator|MakeRotator 0.0 0.0 (* (Math|Float|Clamp(Float) (Variables|Default|GetDoor%20Open%20Angle) 0.0 1.2e+02) -1.0)) false false))

(fn KeyPickUp
  (switch Utilities|FlowControl|Switch|SwitchonEN_DoorStatus (Variables|Default|GetDoorStatus)
    (:NewEnumerator3
      (Variables|Default|SetDoorStatus "NewEnumerator2")
      (Variables|Default|SetIt%20Lock? false))))