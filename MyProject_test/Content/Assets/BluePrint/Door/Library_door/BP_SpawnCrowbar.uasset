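; BP_SpawnCrowbar is a two-trigger actor that spawns a crowbar once, tied to game objective progress.
; Box1 arms it when the third-person character overlaps while the BP_GameManager objective ID, read from a reference cached on BeginPlay, is 6.
; Once armed, any overlap on Box passes through a DoOnce and spawns BP_Crowbar at the Arrow component's location.
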(event OnComponentBeginOverlap(Box1)
  (params (OverlappedComponent :type Primitive%20Component%20Object%20Reference) (OtherActor :type Actor%20Object%20Reference) (OtherComp :type Primitive%20Component%20Object%20Reference) (OtherBodyIndex :type Integer) (bFromSweep :type Boolean) (SweepResult :type Hit%20Result%20Structure%20%28by%20ref%29))
  (Utilities|Casting|CastToBP_ThirdPersonCharacter OtherActor)
  (if (== (Variables|/Game/ThirdPerson/Blueprints/BP_Objective/BP_GameManager.BP_GameManager_C|GetCurrentObjectiveID (Variables|Default|GetAs%20Game%20Manager)) 6)
    (Variables|Default|SetsetBool true)))

(event OnComponentBeginOverlap(Box)
  (params (OverlappedComponent :type Primitive%20Component%20Object%20Reference) (OtherActor :type Actor%20Object%20Reference) (OtherComp :type Primitive%20Component%20Object%20Reference) (OtherBodyIndex :type Integer) (bFromSweep :type Boolean) (SweepResult :type Hit%20Result%20Structure%20%28by%20ref%29))
  (if (Variables|Default|GetsetBool)
    (Utilities|FlowControl|DoOnce false
      (:Completed
        (Game|SpawnActorfromClass "/Game/Assets/BluePrint/Door/Library_door/BP_Crowbar.BP_Crowbar_C" (Math|Transform|MakeTransform (Transformation|GetWorldLocation (Variables|Default|GetArrow)) "0, 0, 0" "1.000000,1.000000,1.000000") "Undefined" "MultiplyWithRoot" 0 0)))))

(event EventBeginPlay
  (bind _returnvalue (Actor|GetActorOfClass "/Game/ThirdPerson/Blueprints/BP_Objective/BP_GameManager.BP_GameManager_C"))
  (Variables|Default|SetAs%20Game%20Manager _returnvalue))

(fn ConstructionScript)