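; BP_Candy is an interactable candy pickup that adds one to the player's inventory candy count.
; It caches the third-person character on BeginPlay, then on CanInteract increments BPCInventory's Candy and destroys itself after a short delay.
; A Sphere overlap with the player shows the inner interact icon and sets the paper sprite's custom depth stencil, reverting both when the overlap ends.
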(event OnComponentBeginOverlap(Sphere)
  (params (OverlappedComponent :type Primitive%20Component%20Object%20Reference) (OtherActor :type Actor%20Object%20Reference) (OtherComp :type Primitive%20Component%20Object%20Reference) (OtherBodyIndex :type Integer) (bFromSweep :type Boolean) (SweepResult :type Hit%20Result%20Structure%20%28by%20ref%29))
  ;[1 1 1] Comment
  (if (== OtherActor (Game|GetPlayerCharacter 0))
    (CallFunction|IconInneron)
    (Rendering|SetCustomDepthStencilValue (Variables|Default|GetPaperSprite) 1)))

(event OnComponentEndOverlap(Sphere)
  (params (OverlappedComponent :type Primitive%20Component%20Object%20Reference) (OtherActor :type Actor%20Object%20Reference) (OtherComp :type Primitive%20Component%20Object%20Reference) (OtherBodyIndex :type Integer))
  ;[1 1 1] Comment
  (if (== OtherActor (Game|GetPlayerCharacter 0))
    (CallFunction|IconInnerOff)
    (Rendering|SetCustomDepthStencilValue (Variables|Default|GetPaperSprite) 0)))

(event Custom|Icon%20innerOn
  ;[1 1 1] Comment
  (Rendering|SetVisibility (Variables|Default|GetinnerInteractIcon) true false))

(event Custom|Icon%20innerOff
  ;[1 1 1] Comment
  (Rendering|SetVisibility (Variables|Default|GetinnerInteractIcon) false false))

(event EventCanInteract
  (bind _as_player (Variables|Default|GetAs%20Player))
  (bind _bpc_inventory (Variables|/Game/ThirdPerson/Blueprints/BP_ThirdPersonCharacter.BP_ThirdPersonCharacter_C|GetBPC_Inventory _as_player))
  ;[1 1 1] Comment
  (Variables|/Game/ThirdPerson/Blueprints/BPC_Inventory.BPC_Inventory_C|SetCandy _bpc_inventory (+ (Variables|/Game/ThirdPerson/Blueprints/BPC_Inventory.BPC_Inventory_C|GetCandy _bpc_inventory) 1))
  (Utilities|FlowControl|Delay 0.2)
  (Actor|DestroyActor))

(event EventBeginPlay
  ;[1 1 1] Get player BP
  (bind _asbp_third_person_character (Utilities|Casting|CastToBP_ThirdPersonCharacter (Game|GetPlayerCharacter 0)))
  (Variables|Default|SetAs%20Player _asbp_third_person_character))

(fn ConstructionScript)