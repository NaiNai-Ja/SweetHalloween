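; BP_Item is a searchable world object that the player searches over a timed interaction.
; Construction-sized outer and inner spheres toggle proximity icons, with the inner also setting an outline stencil.
; CanInteract disables player input, shows WB_Interact and runs a recursive Delay counter, while the widget listens for Interact to cancel.
; Completion removes the widget, hides cues, marks it searched and calls an empty GetKey event, without re-enabling input.
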(event OnComponentBeginOverlap(InnerSphereCollsion)
  (params (OverlappedComponent :type Primitive%20Component%20Object%20Reference) (OtherActor :type Actor%20Object%20Reference) (OtherComp :type Primitive%20Component%20Object%20Reference) (OtherBodyIndex :type Integer) (bFromSweep :type Boolean) (SweepResult :type Hit%20Result%20Structure%20%28by%20ref%29))
  ;[1 1 1] Inner
  (if (not (Variables|Default|GetSearched?))
    (if (== OtherActor (Game|GetPlayerCharacter 0))
      (Utilities|FlowControl|Sequence
        (:then_0
          (CallFunction|OutlineInneron))
        (:then_1
          (CallFunction|IconInneron))))))

(event OnComponentEndOverlap(InnerSphereCollsion)
  (params (OverlappedComponent :type Primitive%20Component%20Object%20Reference) (OtherActor :type Actor%20Object%20Reference) (OtherComp :type Primitive%20Component%20Object%20Reference) (OtherBodyIndex :type Integer))
  ;[1 1 1] Inner
  (if (== OtherActor (Game|GetPlayerCharacter 0))
    (Utilities|FlowControl|Sequence
      (:then_0
        (CallFunction|OutlineInnerOff))
      (:then_1
        (CallFunction|IconInnerOff)))))

(event OnComponentBeginOverlap(OuterSphereCollsion)
  (params (OverlappedComponent :type Primitive%20Component%20Object%20Reference) (OtherActor :type Actor%20Object%20Reference) (OtherComp :type Primitive%20Component%20Object%20Reference) (OtherBodyIndex :type Integer) (bFromSweep :type Boolean) (SweepResult :type Hit%20Result%20Structure%20%28by%20ref%29))
  ;[1 1 1] Outer
  (if (not (Variables|Default|GetSearched?))
    (if (== OtherActor (Game|GetPlayerCharacter 0))
      (CallFunction|IconOuteron))))

(event OnComponentEndOverlap(OuterSphereCollsion)
  (params (OverlappedComponent :type Primitive%20Component%20Object%20Reference) (OtherActor :type Actor%20Object%20Reference) (OtherComp :type Primitive%20Component%20Object%20Reference) (OtherBodyIndex :type Integer))
  ;[1 1 1] Outer
  (if (== OtherActor (Game|GetPlayerCharacter 0))
    (CallFunction|IconOuterOff)))

(event Custom|Searching
  ;[1 1 1] Searching
  (bind _returnvalue (UserInterface|CreateWidget "/Game/UI/WB_Interact.WB_Interact_C"))
  (bind _output_get (Variables|Default|SetHoldButtomRef _returnvalue))
  (UserInterface|Viewport|AddtoViewport _output_get 0)
  (Input|DisableInput (Variables|Default|GetAs%20BP%20Third%20Person%20Character) 0))

(event Custom|Icon%20innerOn
  ;[1 1 1] Comment
  (Rendering|SetVisibility (Variables|Default|GetinnerInteractIcon) true false)
  (Rendering|SetVisibility (Variables|Default|GetouterInteractIcon) false false))

(event Custom|Icon%20OuterOn
  ;[1 1 1] Comment
  (Rendering|SetVisibility (Variables|Default|GetouterInteractIcon) true false))

(event Custom|Get%20Key)

(event Custom|Stop%20Searching
  ;[1 1 1] Comment
  (Widget|RemovefromParent (Variables|Default|GetHoldButtomRef))
  (Input|EnableInput (Variables|Default|GetAs%20BP%20Third%20Person%20Character) 0)
  (Variables|Default|SetCancel? true))

(event Custom|Icon%20innerOff
  ;[1 1 1] Comment
  (Rendering|SetVisibility (Variables|Default|GetinnerInteractIcon) false false)
  (Rendering|SetVisibility (Variables|Default|GetouterInteractIcon) true false))

(event Custom|Interact%20Time%20In%20Item
  ;[1 1 1] Comment
  (if (Variables|Default|GetCancel?)
    (Development|PrintString "Cancel")
    (Variables|Default|SetCount 0.0)
    (elif (< (Variables|Default|GetCount) 1e+02)
      (Utilities|FlowControl|Delay 1.25)
      (Variables|Default|SetCount (+ (Variables|Default|GetCount) 25.0))
      (CallFunction|InteractTimeinItem)
      (else
        (Development|PrintString "Completed")
        (Variables|Default|SetCount 0.0)
        (Widget|RemovefromParent (Variables|Default|GetHoldButtomRef))
        (Variables|Default|SetSearched? true)
        (Utilities|FlowControl|Sequence
          (:then_0
            (CallFunction|OutlineInnerOff)
            (CallFunction|IconInnerOff)
            (CallFunction|IconOuterOff))
          (:then_1
            (Variables|Default|SetBox%20Status "NewEnumerator1"))
          (:then_2
            (CallFunction|GetKey)))))))

(event Custom|Outline%20innerOn
  ;[1 1 1] Comment
  (Rendering|SetCustomDepthStencilValue (Variables|Default|GetStaticMesh) 1))

(event Custom|Outline%20innerOff
  ;[1 1 1] Comment
  (Rendering|SetCustomDepthStencilValue (Variables|Default|GetStaticMesh) 0))

(event Custom|Icon%20OuterOff
  ;[1 1 1] Comment
  (Rendering|SetVisibility (Variables|Default|GetouterInteractIcon) false false))

(event EventBeginPlay
  ;[1 1 1] Get player
  (bind _asbp_third_person_character (Utilities|Casting|CastToBP_ThirdPersonCharacter (Game|GetPlayerCharacter 0)))
  (Variables|Default|SetAs%20BP%20Third%20Person%20Character _asbp_third_person_character))

(event EventCanInteract
  ;[1 1 1] Comment
  (switch Utilities|FlowControl|Switch|SwitchonEN_BoxStatus (Variables|Default|GetBox%20Status)
    (:NewEnumerator0
      (CallFunction|Searching)
      (CallFunction|InteractTimeinItem)
      (Class|UserWidget|ListenforInputAction (Variables|Default|GetHoldButtomRef) "Interact" "IE_Pressed" true (delegate Custom|Stop%20Searching)))))

(fn ConstructionScript
  (Components|Sphere|SetSphereRadius (Variables|Default|GetInnerSphereCollsion) (Variables|Public|GetInnerSphereRadius) true)
  (Components|Sphere|SetSphereRadius (Variables|Default|GetOuterSphereCollsion) (Variables|Public|GetOuterSphereRadius) true))