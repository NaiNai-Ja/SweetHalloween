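; BP_Item is an interactable world item that signals when the player is near or within reach.
; An outer sphere shows a distant icon; an inner sphere swaps icons, changes the mesh's custom depth stencil and sets the character's CanInteract and InteractWith.
; Exits revert these, Searched blocks new prompts, and construction applies both configurable radii.
; The Interact input only prints a placeholder message; Searched is never set here.
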(event OnComponentBeginOverlap(InnerSphereCollsion)
  (params (OverlappedComponent :type Primitive%20Component%20Object%20Reference) (OtherActor :type Actor%20Object%20Reference) (OtherComp :type Primitive%20Component%20Object%20Reference) (OtherBodyIndex :type Integer) (bFromSweep :type Boolean) (SweepResult :type Hit%20Result%20Structure%20%28by%20ref%29))
  (bind _as_bp_third_person_character (Variables|Default|GetAs%20BP%20Third%20Person%20Character))
  ;[1 1 1] Inner
  (if (not (Variables|Default|GetSearched?))
    (if (== OtherActor (Game|GetPlayerCharacter 0))
      (Utilities|FlowControl|Sequence
        (:then_0
          (Rendering|SetCustomDepthStencilValue (Variables|Default|GetStaticMesh) 1)
          (Variables|/Game/ThirdPerson/Blueprints/BP_ThirdPersonCharacter.BP_ThirdPersonCharacter_C|SetCan%20Interact _as_bp_third_person_character true)
          (Variables|/Game/ThirdPerson/Blueprints/BP_ThirdPersonCharacter.BP_ThirdPersonCharacter_C|Setinteract%20with _as_bp_third_person_character 2.0))
        (:then_1
          (Rendering|SetVisibility (Variables|Default|GetinnerInteractIcon) true false)
          (Rendering|SetVisibility (Variables|Default|GetouterInteractIcon) false false))))))

(event OnComponentEndOverlap(InnerSphereCollsion)
  (params (OverlappedComponent :type Primitive%20Component%20Object%20Reference) (OtherActor :type Actor%20Object%20Reference) (OtherComp :type Primitive%20Component%20Object%20Reference) (OtherBodyIndex :type Integer))
  (bind _as_bp_third_person_character (Variables|Default|GetAs%20BP%20Third%20Person%20Character))
  ;[1 1 1] Inner
  (if (== OtherActor (Game|GetPlayerCharacter 0))
    (Utilities|FlowControl|Sequence
      (:then_0
        (Rendering|SetCustomDepthStencilValue (Variables|Default|GetStaticMesh) 0)
        (Variables|/Game/ThirdPerson/Blueprints/BP_ThirdPersonCharacter.BP_ThirdPersonCharacter_C|SetCan%20Interact _as_bp_third_person_character false)
        (Variables|/Game/ThirdPerson/Blueprints/BP_ThirdPersonCharacter.BP_ThirdPersonCharacter_C|Setinteract%20with _as_bp_third_person_character 0.0))
      (:then_1
        (Rendering|SetVisibility (Variables|Default|GetinnerInteractIcon) false false)
        (Rendering|SetVisibility (Variables|Default|GetouterInteractIcon) true false)))))

(event OnComponentBeginOverlap(OuterSphereCollsion)
  (params (OverlappedComponent :type Primitive%20Component%20Object%20Reference) (OtherActor :type Actor%20Object%20Reference) (OtherComp :type Primitive%20Component%20Object%20Reference) (OtherBodyIndex :type Integer) (bFromSweep :type Boolean) (SweepResult :type Hit%20Result%20Structure%20%28by%20ref%29))
  ;[1 1 1] Outer
  (if (not (Variables|Default|GetSearched?))
    (if (== OtherActor (Game|GetPlayerCharacter 0))
      (Rendering|SetVisibility (Variables|Default|GetouterInteractIcon) true false))))

(event OnComponentEndOverlap(OuterSphereCollsion)
  (params (OverlappedComponent :type Primitive%20Component%20Object%20Reference) (OtherActor :type Actor%20Object%20Reference) (OtherComp :type Primitive%20Component%20Object%20Reference) (OtherBodyIndex :type Integer))
  ;[1 1 1] Outer
  (if (== OtherActor (Game|GetPlayerCharacter 0))
    (Rendering|SetVisibility (Variables|Default|GetouterInteractIcon) false false)))

(event EventBeginPlay
  ;[1 1 1] Get player
  (bind _asbp_third_person_character (Utilities|Casting|CastToBP_ThirdPersonCharacter (Game|GetPlayerCharacter 0)))
  (Variables|Default|SetAs%20BP%20Third%20Person%20Character _asbp_third_person_character))

(event Input|ActionEvents|InputActionInteract
  (params (Key :type Key%20Structure :default "None"))
  ;[1 1 1] Inner
  (:Pressed
    (Development|PrintString "Hello")))

(fn ConstructionScript
  (Components|Sphere|SetSphereRadius (Variables|Default|GetInnerSphereCollsion) (Variables|Public|GetInnerSphereRadius) true)
  (Components|Sphere|SetSphereRadius (Variables|Default|GetOuterSphereCollsion) (Variables|Public|GetOuterSphereRadius) true))