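; BP_Objective is a pickup trigger that assigns its objective to the player character on overlap.
; Its Box overlap casts the other actor to BP_ThirdPersonCharacter and acts only if that character is not already on an objective.
; It then sets the character's CurrentObjective and IsOnObjective flag, plays a 2D ping sound and destroys itself.
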(event OnComponentBeginOverlap(Box)
  (params (OverlappedComponent :type Primitive%20Component%20Object%20Reference) (OtherActor :type Actor%20Object%20Reference) (OtherComp :type Primitive%20Component%20Object%20Reference) (OtherBodyIndex :type Integer) (bFromSweep :type Boolean) (SweepResult :type Hit%20Result%20Structure%20%28by%20ref%29))
  ;[1 1 1] BP_Character
  (bind _asbp_third_person_character (Utilities|Casting|CastToBP_ThirdPersonCharacter OtherActor))
  (Variables|Default|SetCharacter%20Ref _asbp_third_person_character)
  (if (not (Variables|/Game/ThirdPerson/Blueprints/BP_ThirdPersonCharacter.BP_ThirdPersonCharacter_C|GetIsOnObjective? (Variables|Default|GetCharacter%20Ref)))
    (Variables|/Game/ThirdPerson/Blueprints/BP_ThirdPersonCharacter.BP_ThirdPersonCharacter_C|SetCurrentObjective (Variables|Default|GetCharacter%20Ref) (Variables|Default|GetObjective))
    (Variables|/Game/ThirdPerson/Blueprints/BP_ThirdPersonCharacter.BP_ThirdPersonCharacter_C|SetIsOnObjective? (Variables|Default|GetCharacter%20Ref) true)
    (Audio|PlaySound2D "/Engine/EngineSounds/1kSineTonePing.1kSineTonePing" 1.0 1.0 0.0 0 0)
    (Actor|DestroyActor)))

(fn ConstructionScript)