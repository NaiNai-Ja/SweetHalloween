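; Enemy AI helper actor that picks whichever of its four arrow markers is closest to the first player character.
; BeginPlay caches the arrow locations and measures each distance to the player; the CheckDistance event measures them again on demand.
; Distance is a RepNotify array whose OnRep scans for the minimum and passes that arrow's location to the Enemy_controller_01 found in the level through its Location call.
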(event Custom|CheckDistance
  (bind _returnvalue (Game|GetPlayerCharacter 0))
  (bind _returnvalue_2 (Transformation|GetActorLocation _returnvalue))
  (Variables|Default|SetDistance (Utilities|Array|MakeArray (Math|Vector|Distance(Vector) (Transformation|GetWorldLocation (Variables|Default|GetArrow1)) _returnvalue_2) (Math|Vector|Distance(Vector) (Transformation|GetWorldLocation (Variables|Default|GetArrow2)) _returnvalue_2) (Math|Vector|Distance(Vector) (Transformation|GetWorldLocation (Variables|Default|GetArrow3)) _returnvalue_2) (Math|Vector|Distance(Vector) (Transformation|GetWorldLocation (Variables|Default|GetArrow4)) _returnvalue_2))))

(event EventBeginPlay
  (bind _returnvalue (Game|GetPlayerCharacter 0))
  (bind _arrow1 (Variables|Default|GetArrow1))
  (bind _arrow4 (Variables|Default|GetArrow4))
  (bind _arrow3 (Variables|Default|GetArrow3))
  (bind _arrow2 (Variables|Default|GetArrow2))
  (bind _returnvalue_2 (Transformation|GetWorldLocation _arrow1))
  (bind _returnvalue_3 (Transformation|GetActorLocation _returnvalue))
  (bind _returnvalue_4 (Transformation|GetWorldLocation _arrow2))
  (bind _returnvalue_5 (Transformation|GetWorldLocation _arrow3))
  (bind _returnvalue_6 (Transformation|GetWorldLocation _arrow4))
  (Variables|Default|SetDistance (Utilities|Array|MakeArray (Math|Vector|Distance(Vector) _returnvalue_2 _returnvalue_3) (Math|Vector|Distance(Vector) _returnvalue_4 _returnvalue_3) (Math|Vector|Distance(Vector) _returnvalue_5 _returnvalue_3) (Math|Vector|Distance(Vector) _returnvalue_6 _returnvalue_3)))
  (Variables|Default|SetArrowLocation (Utilities|Array|MakeArray _returnvalue_2 _returnvalue_4 _returnvalue_5 _returnvalue_6)))

(fn ConstructionScript)

(fn OnRepDistance
  (Variables|Default|SetMinDistance (Utilities|Array|Get(acopy) (Variables|Default|GetDistance)))
  (for (_array_element _array_index) (Variables|Default|GetDistance)
    (if (<= _array_element (Variables|Default|GetMinDistance))
      (Variables|Default|SetMinDistance _array_element)
      (Variables|Default|SetMinLocation (Utilities|Array|Get(acopy) (Variables|Default|GetArrowLocation) _array_index))))
  (bind _returnvalue (Actor|GetActorOfClass "/Game/Characters/BP_Enemy_01/AI_BP_01/Enemy_controller_01.Enemy_controller_01_C"))
  (Default|Location _returnvalue (Variables|Default|GetMinLocation)))