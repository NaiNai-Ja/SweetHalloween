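; BP_Enemy_01 is an enemy that fades in when the player enters its Sphere and fades out on exit.
; A reversible Timeline drives the "Mash Opacity" scalar in the shared MPC_Enemy_01 parameter collection.
; Tick copies PlayerMind from the player's status component into a RepNotify variable.
; Its OnRep sets the AI Blackboard key "PlayerSane?" true at or below a low mind threshold, false above it.
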(event OnComponentBeginOverlap(Sphere)
  (params (OverlappedComponent :type Primitive%20Component%20Object%20Reference) (OtherActor :type Actor%20Object%20Reference) (OtherComp :type Primitive%20Component%20Object%20Reference) (OtherBodyIndex :type Integer) (bFromSweep :type Boolean) (SweepResult :type Hit%20Result%20Structure%20%28by%20ref%29))
  (if (== OtherActor (Variables|Default|GetAs%20BP_Player))
    (CallFunction|ShowItself)
    (Actor|GetActorOfClass "/Game/Characters/BP_Enemy_01/AI_BP_01/Enemy_controller_01.Enemy_controller_01_C")))

(event OnComponentEndOverlap(Sphere)
  (params (OverlappedComponent :type Primitive%20Component%20Object%20Reference) (OtherActor :type Actor%20Object%20Reference) (OtherComp :type Primitive%20Component%20Object%20Reference) (OtherBodyIndex :type Integer))
  (if (== OtherActor (Variables|Default|GetAs%20BP_Player))
    (CallFunction|HideItSelf)))

(event Custom|Hide%20it%20self
  (bind _showandhide (Timeline|Timeline Reverse)
    (:Update
      (Rendering|Material|SetScalarParameterValue "/Game/Characters/BP_Enemy_01/Model_Enemy_1/MPC_Enemy_01.MPC_Enemy_01" "Mash Opacity" (Math|Float|Lerp 0.0 1.0 _showandhide) :!class /Script/Engine.KismetMaterialLibrary))))

(event Custom|ShowItself
  (bind _showandhide (Timeline|Timeline Play)
    (:Update
      (Rendering|Material|SetScalarParameterValue "/Game/Characters/BP_Enemy_01/Model_Enemy_1/MPC_Enemy_01.MPC_Enemy_01" "Mash Opacity" (Math|Float|Lerp 0.0 1.0 _showandhide) :!class /Script/Engine.KismetMaterialLibrary))))

(event EventTick
  (params (DeltaSeconds :type Float%20%28single-precision%29))
  (Variables|Default|SetGetPlayermind (Variables|/Game/ThirdPerson/Blueprints/BPC_PlayerStatus.BPC_PlayerStatus_C|GetPlayer%20Mind (Variables|/Game/ThirdPerson/Blueprints/BP_ThirdPersonCharacter.BP_ThirdPersonCharacter_C|GetBPC_PlayerStatus (Variables|Default|GetAs%20BP_Player)))))

(event EventBeginPlay
  (bind _asbp_third_person_character (Utilities|Casting|CastToBP_ThirdPersonCharacter (Game|GetPlayerCharacter 0)))
  (bind _output_get (Variables|Default|SetAs%20BP_Player _asbp_third_person_character))
  (Variables|Default|SetGetPlayermind (Variables|/Game/ThirdPerson/Blueprints/BPC_PlayerStatus.BPC_PlayerStatus_C|GetPlayer%20Mind (Variables|/Game/ThirdPerson/Blueprints/BP_ThirdPersonCharacter.BP_ThirdPersonCharacter_C|GetBPC_PlayerStatus _output_get)))
  (CallFunction|HideItSelf))

(fn ConstructionScript)

(fn OnRepGetPlayermind
  (bind _returnvalue (Utilities|Name|MakeLiteralName "PlayerSane?"))
  (bind _self self)
  (bind _returnvalue_2 (AI|GetAIController _self))
  (bind _returnvalue_3 (AI|GetBlackboard _returnvalue_2))
  (if (<= (Variables|Default|GetGetPlayermind) 0.2)
    (AI|Components|Blackboard|SetValueasBool _returnvalue_3 _returnvalue true)
    (else
      (AI|Components|Blackboard|SetValueasBool _returnvalue_3 _returnvalue false))))