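; BP_SpawnEnemy_2 is a location provider that hands random points to Enemy_controller_02.
; On BeginPlay it caches the world locations of four Arrow components in the SpawnEnemy2 array.
; Its RandomLocatiom event finds the controller with GetActorOfClass and passes a random entry to GetNewLocation.
; RandomInteger(3) yields only indices 0 to 2, so the fourth arrow is never chosen.
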(event Custom|RandomLocatiom
  (bind _returnvalue (Actor|GetActorOfClass "/Game/Characters/BP_Enemy_02/AI_BP_02/Enemy_controller_02.Enemy_controller_02_C"))
  (Default|GetNewLocation _returnvalue (Utilities|Array|Get(acopy) (Variables|Default|GetSpawnEnemy_2) (Math|Random|RandomInteger 3))))

(event EventBeginPlay
  (Variables|Default|SetSpawnEnemy_2 (Utilities|Array|MakeArray (Transformation|GetWorldLocation (Variables|Default|GetArrow1)) (Transformation|GetWorldLocation (Variables|Default|GetArrow2)) (Transformation|GetWorldLocation (Variables|Default|GetArrow3)) (Transformation|GetWorldLocation (Variables|Default|GetArrow4)))))

(fn ConstructionScript)