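; BP_Enemy_02 is an AI enemy whose material opacity and blackboard state follow the player's PlayerMind stat.
; It copies PlayerMind from the player's status component every Tick into a RepNotify variable, which drives MPC_Enemy_01 opacity inversely and sets "PlayerSane?" true at or below a low threshold.
; PawnSensing sets "SeePlayer?" true on sighting the player, then sets it true again after a retriggerable delay, never clearing it.
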(event OnSeePawn(PawnSensing)
  (params (Pawn :type Pawn%20Object%20Reference))
  (bind _returnvalue (Utilities|Name|MakeLiteralName "SeePlayer?"))
  (bind _self self)
  (bind _returnvalue_2 (AI|GetAIController _self))
  (bind _returnvalue_3 (AI|GetBlackboard _returnvalue_2))
  (if (== Pawn (Variables|Default|GetAs%20BP_Player))
    (AI|Components|Blackboard|SetValueasBool _returnvalue_3 _returnvalue true)
    (Utilities|FlowControl|RetriggerableDelay 2.0)
    (AI|Components|Blackboard|SetValueasBool _returnvalue_3 _returnvalue true)))

(event EventTick
  (params (DeltaSeconds :type Float%20%28single-precision%29))
  (Variables|Default|SetGetPlayermind (Variables|/Game/ThirdPerson/Blueprints/BPC_PlayerStatus.BPC_PlayerStatus_C|GetPlayer%20Mind (Variables|/Game/ThirdPerson/Blueprints/BP_ThirdPersonCharacter.BP_ThirdPersonCharacter_C|GetBPC_PlayerStatus (Variables|Default|GetAs%20BP_Player)))))

(event EventBeginPlay
  (bind _asbp_third_person_character (Utilities|Casting|CastToBP_ThirdPersonCharacter (Game|GetPlayerCharacter 0)))
  (bind _output_get (Variables|Default|SetAs%20BP_Player _asbp_third_person_character))
  (Variables|Default|SetGetPlayermind (Variables|/Game/ThirdPerson/Blueprints/BPC_PlayerStatus.BPC_PlayerStatus_C|GetPlayer%20Mind (Variables|/Game/ThirdPerson/Blueprints/BP_ThirdPersonCharacter.BP_ThirdPersonCharacter_C|GetBPC_PlayerStatus _output_get))))

(fn ConstructionScript)

(fn OnRepGetPlayermind
  (bind _returnvalue (Utilities|Name|MakeLiteralName "PlayerSane?"))
  (bind _self self)
  (bind _returnvalue_2 (AI|GetAIController _self))
  (bind _returnvalue_3 (AI|GetBlackboard _returnvalue_2))
  (Utilities|FlowControl|Sequence
    (:then_0
      (Rendering|Material|SetScalarParameterValue "/Game/Characters/BP_Enemy_01/MPC_Enemy_01.MPC_Enemy_01" "Mash Opacity" (- 1.0 (Variables|Default|GetGetPlayermind)) :!class /Script/Engine.KismetMaterialLibrary))
    (:then_1
      (if (<= (Variables|Default|GetGetPlayermind) 0.2)
        (AI|Components|Blackboard|SetValueasBool _returnvalue_3 _returnvalue true)
        (else
          (AI|Components|Blackboard|SetValueasBool _returnvalue_3 _returnvalue false))))))