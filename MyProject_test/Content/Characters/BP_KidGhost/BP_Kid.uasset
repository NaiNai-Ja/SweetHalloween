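; BP_Kid is a ghost child character the player interacts with to toggle between following and staying.
; While following, it uses AI MoveTo toward the player, re-issued on success only while the player's Mind is at most 0.8.
; A recursive delay loop blinks an icon faster the nearer the kid gets to a BP_Point.
; Tick drives a material parameter collection's opacity inversely from Mind.
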(event Custom|FollowPlayer
  ;[1 1 1] Comment
  (if (Variables|Default|GetFollower)
    (if (<= (Variables|/Game/ThirdPerson/Blueprints/BP_ThirdPersonCharacter.BP_ThirdPersonCharacter_C|GetMind (Variables|Default|GetAs%20BP%20Third%20Person%20Character)) 0.8)
      (AI|AIMoveTo self "0, 0, 0" (Game|GetPlayerCharacter 0) 1.5e+02 false
        (:OnSuccess
          (CallFunction|FollowPlayer))))))

(event Custom|LengthToPoint
  (bind _delaytime (Variables|Default|GetDelayTime))
  (if (Variables|Default|GetFollower)
    (CallFunction|SetDelayTime)
    (CallFunction|Iconon)
    (Utilities|FlowControl|Delay _delaytime)
    (CallFunction|IconOff)
    (Utilities|FlowControl|Delay _delaytime)
    (CallFunction|LengthtoPoint)
    (else
      (CallFunction|IconOff))))

(event Custom|Icon%20Off
  ;[1 1 1] Comment
  (Rendering|SetVisibility (Variables|Default|GetIcon) false false))

(event Custom|Icon%20On
  ;[1 1 1] Comment
  (Rendering|SetVisibility (Variables|Default|GetIcon) true false))

(event Custom|Set%20Delay%20Time
  (bind _point (Variables|Default|GetPoint))
  (bind _returnvalue (Transformation|GetDistanceTo _point))
  (if (Variables|Default|GetFollower)
    (if (< _returnvalue 5e+02)
      (Variables|Default|SetDelayTime 0.1)
      (elif (< _returnvalue 7.5e+02)
        (Variables|Default|SetDelayTime 1.0)
        (elif (< _returnvalue 1e+03)
          (Variables|Default|SetDelayTime 2.0)
          (else
            (Variables|Default|SetDelayTime 3.0)))))))

(event EventCanInteract
  ;[1 1 1] Comment
  (switch Utilities|FlowControl|Switch|SwitchonEN_GK (Variables|Default|GetGKstatus)
    (:NewEnumerator0
      (Variables|Default|SetGKstatus "NewEnumerator1")
      (Variables|Default|SetFollower true)
      (CallFunction|FollowPlayer)
      (CallFunction|LengthtoPoint))
    (:NewEnumerator1
      (Variables|Default|SetGKstatus "NewEnumerator0")
      (Development|PrintString "Stay")
      (Variables|Default|SetFollower false))))

(event EventBeginPlay
  ;[1 1 1] Comment
  (Utilities|FlowControl|Sequence
    (:then_0
      (bind _asbp_third_person_character (Utilities|Casting|CastToBP_ThirdPersonCharacter (Game|GetPlayerCharacter 0)))
      (Variables|Default|SetAs%20BP%20Third%20Person%20Character _asbp_third_person_character))
    (:then_1
      (CallFunction|IconOff)
      (bind _returnvalue (Actor|GetActorOfClass "/Game/Characters/BP_KidGhost/BP_Point.BP_Point_C"))
      (Variables|Default|SetPoint _returnvalue))))

(event EventTick
  (params (DeltaSeconds :type Float%20%28single-precision%29))
  ;[1 1 1] Comment
  (Rendering|Material|SetScalarParameterValue "/Game/Characters/BP_KidGhost/MPC_InvisKid.MPC_InvisKid" "Mash Opacity" (- 1.25 (Variables|/Game/ThirdPerson/Blueprints/BP_ThirdPersonCharacter.BP_ThirdPersonCharacter_C|GetMind (Variables|Default|GetAs%20BP%20Third%20Person%20Character))) :!class /Script/Engine.KismetMaterialLibrary))

(fn ConstructionScript)