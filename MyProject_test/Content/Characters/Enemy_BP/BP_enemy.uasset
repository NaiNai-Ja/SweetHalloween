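; Enemy ghost that appears and hunts the player as their PlayerMind stat drops.
; Each Tick writes inverse PlayerMind to an MPC_Tutorial opacity parameter, fading the ghost in as it falls.
; Low PlayerMind sets a Hunt flag driving AIMoveTo toward the player and repeats a delayed crying sound.
; Hunt clears when PlayerMind recovers or PawnSensing sees a non-player pawn.
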(event OnSeePawn(PawnSensing)
  (params (Pawn :type Pawn%20Object%20Reference))
  (if (not (== Pawn (Game|GetPlayerCharacter 0)))
    (Variables|Default|Sethunt false)))

(event EventTick
  (params (DeltaSeconds :type Float%20%28single-precision%29))
  (bind _returnvalue (Game|GetPlayerCharacter 0))
  (Utilities|FlowControl|Sequence
    (:then_0
      (if (Variables|Default|Gethunt)
        (AI|AIMoveTo self "0, 0, 0" _returnvalue 1e+01 false
          (:then
            (Utilities|FlowControl|RetriggerableDelay 5.0)))))
    (:then_1
      (bind _asbp_third_person_character (Utilities|Casting|CastToBP_ThirdPersonCharacter _returnvalue))
      (Rendering|Material|SetScalarParameterValue "/Game/Characters/Enemy_BP/MPC_Tutorial.MPC_Tutorial" "Mash Opacity" (- 1.0 (Variables|/Game/ThirdPerson/Blueprints/BPC_PlayerStatus.BPC_PlayerStatus_C|GetPlayer%20Mind (Variables|/Game/ThirdPerson/Blueprints/BP_ThirdPersonCharacter.BP_ThirdPersonCharacter_C|GetBPC_PlayerStatus _asbp_third_person_character))) :!class /Script/Engine.KismetMaterialLibrary)
      (if (<= (Variables|/Game/ThirdPerson/Blueprints/BPC_PlayerStatus.BPC_PlayerStatus_C|GetPlayer%20Mind (Variables|/Game/ThirdPerson/Blueprints/BP_ThirdPersonCharacter.BP_ThirdPersonCharacter_C|GetBPC_PlayerStatus _asbp_third_person_character)) 0.2)
        (Variables|Default|Sethunt true)
        (Utilities|FlowControl|RetriggerableDelay 3.0)
        (Variables|Default|Sethunt false)
        (else
          (Variables|Default|Sethunt false))))
    (:then_2
      (if (<= (Variables|/Game/ThirdPerson/Blueprints/BPC_PlayerStatus.BPC_PlayerStatus_C|GetPlayer%20Mind (Variables|/Game/ThirdPerson/Blueprints/BP_ThirdPersonCharacter.BP_ThirdPersonCharacter_C|GetBPC_PlayerStatus _asbp_third_person_character)) 0.2)
        (Utilities|FlowControl|Delay 5.0)
        (Audio|PlaySoundatLocation "/Game/Sounds/Forlay/SFX_Trigger_Ghostcrying.SFX_Trigger_Ghostcrying" (Transformation|GetActorLocation) "0, 0, 0" 0.2 1.0 0.0 0 0 0 0)))))

(fn ConstructionScript)